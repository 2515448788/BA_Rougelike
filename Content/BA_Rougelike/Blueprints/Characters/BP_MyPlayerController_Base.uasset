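; Base player controller that creates the main HUD canvas and drives lock-on targeting for the controlled pawn.
; Other code sets, clears and reads the current target and the canvas through accessor functions.
; Each tick, while the target is alive, it eases control yaw toward it with RInterpTo from the pawn's rotation.
; It also messages the pawn to switch rotate mode, reverting when the target is missing or dead.
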(event `self.ReceiveBeginPlay`
  (set `self.bShowMouseCursor` false)
  (`self.InitHUD`))

(event `self.ReceiveTick`
  (params (DeltaSeconds :type "Float (single-precision)"))
  (set `self.Delta Seconds` DeltaSeconds)
  (bind _targetactor (`self.TargetActor`)
    (:`then`
      (`self.LookAtTargetActor` _targetactor))
    (:`else`
      (message `/Game/BA_Rougelike/Blueprints/BPI/BPI_PlayerCharacter.Set_RotateMode` (`self.K2_GetPawn`) "NewEnumerator0"))))

(event `/Game/BA_Rougelike/Blueprints/BPI/BPI_PlayerController.Set_CurrentTarget`
  (params (TargetActor :type "Actor Object Reference"))
  (set `self.TargetActor` TargetActor))

(event `/Game/BA_Rougelike/Blueprints/BPI/BPI_PlayerController.Clear_CurrentTarget`
  (set `self.TargetActor` null))

(fn `Get_BaseCanvas`
  (returns (UserBaseCanvas :type "/Game/BA_Rougelike/Blueprints/UMG/WBP_UserBaseCanvas Object Reference"))
  (return (`self.UserBaseCanvans`)))

(fn `Get_CurrentTarget`
  (returns (CurTarget :type "Actor Object Reference"))
  (return (`self.TargetActor`)))

(fn `InitHUD`
  (bind _returnvalue (`|CreateWidget` "/Game/BA_Rougelike/Blueprints/UMG/WBP_UserBaseCanvas.WBP_UserBaseCanvas_C"))
  (bind _output_get (set `self.UserBaseCanvans` _returnvalue))
  (`UserWidget.AddToViewport` _output_get 0))

(fn `LookAtTargetActor`
  (params (TargetActor :type "Actor Object Reference"))
  (bind (_returnvalue_roll _returnvalue_pitch) (`KismetMathLibrary.BreakRotator` (`self.GetControlRotation`)))
  (bind (_returnvalue_roll_2 _returnvalue_pitch_2 _returnvalue_yaw) (`KismetMathLibrary.BreakRotator` (`KismetMathLibrary.RInterpTo` (`self.K2_GetActorRotation` (`self.K2_GetPawn`)) (`KismetMathLibrary.FindLookAtRotation` (`self.K2_GetActorLocation` (`self.K2_GetPawn`)) (`self.K2_GetActorLocation` TargetActor)) (`self.Delta Seconds`) 8.0)))
  (`/Engine/EditorBlueprintResources/StandardMacros.IsValid` TargetActor
    (:`Is Valid`
      (`self.IsTargetAlive` (`local.TargetActor`)
        (:`真`
          (`self.SetControlRotation` (`KismetMathLibrary.MakeRotator` _returnvalue_roll _returnvalue_pitch _returnvalue_yaw))
          (message `/Game/BA_Rougelike/Blueprints/BPI/BPI_PlayerCharacter.Set_RotateMode` (`self.K2_GetPawn`) "NewEnumerator1"))
        (:`false`
          (message `/Game/BA_Rougelike/Blueprints/BPI/BPI_PlayerCharacter.Set_RotateMode` (`self.K2_GetPawn`) "NewEnumerator0" :!label _label))))
    (:`Is Not Valid`
      (goto _label))))

(fn `UserConstructionScript`)