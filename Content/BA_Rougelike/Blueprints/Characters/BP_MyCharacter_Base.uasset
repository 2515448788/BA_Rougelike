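; Base player character for a roguelike with camera-relative movement and automatic attacks on enemies in range.
; A looping timer overlaps pawns, filters by group and health, and passes the nearest target to the controller unless switching is locked.
; A second timer starts the montage and fire sound once both forward vectors oppose.
; GAS supplies starting abilities, effects and stats, and converts incoming damage into a SetByCaller effect.
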(event `self.ReceiveBeginPlay`
  ;[1 1 1] 初始化
  (`self.InitMappingContext`) ; 初始化输入
  (`self.BindAttributeChangeFun`) ; 绑定属性变化回调
  (`self.InitBasicGAGE`) ; 给予基础GA 应用基础GE
  (`self.InitGroupMap`) ; 注册到角色组子系统
  (`self.StartLoopCheckTarget`) ; 开始循环检测敌人
  (`self.OnBeginPlayComplete`) ; 广播初始化完成
)

(event `EnhancedInput|/Game/ThirdPerson/Input/Actions/IA_Move`
  (params (ActionValue :type "Vector2D Structure") (ElapsedSeconds :type "Float (double-precision)") (TriggeredSeconds :type "Float (double-precision)") (InputAction :type "InputAction Object Reference" :default "/Game/ThirdPerson/Input/Actions/IA_Move.IA_Move"))
  ;[1 1 1] 移动
  (:`Triggered`
    (`self.AddMovementInput` (`SceneComponent.GetRightVector` (`self.Camera`)) ActionValue_X)
    (`self.AddMovementInput` (`SceneComponent.GetForwardVector` (`self.Camera`)) ActionValue_Y)))

(event `self.ReceiveTick`
  (params (DeltaSeconds :type "Float (single-precision)"))
  ;[1 1 1] TICK
  (`self.Debug_TargetSystem`))

(event `EnhancedInput|/Game/BA_Rougelike/Input/Actions/IA_Debug_ShowAttributeSet`
  (params (ActionValue :type Boolean) (ElapsedSeconds :type "Float (double-precision)") (TriggeredSeconds :type "Float (double-precision)") (InputAction :type "InputAction Object Reference" :default "/Game/BA_Rougelike/Input/Actions/IA_Debug_ShowAttributeSet.IA_Debug_ShowAttributeSet"))
  (bind _returnvalue (`GameplayStatics.GetPlayerController` 0))
  ;[1 1 1] 调试-显示所有属性
  (:`Started`
    (switch `/Game/BA_Rougelike/GameData/Enums/Character/Debug/E_DebugMode` (`self.DebugMode_AttributeSet`)
      (:`NewEnumerator2`
        (set `self.DebugMode_AttributeSet` "NewEnumerator1")
        (bind _userbasecanvas (message `/Game/BA_Rougelike/Blueprints/BPI/BPI_PlayerController.Get_BaseCanvas` (`self.GetController`)))
        (bind _returnvalue_2 (`/Game/BA_Rougelike/Blueprints/UMG/WBP_UserBaseCanvas.PushWidget` _userbasecanvas "/Game/BA_Rougelike/Blueprints/UMG/Debug/CAW_AttributeSetPanel.CAW_AttributeSetPanel_C"))
        (set `self.AttributeSetPanel` _returnvalue_2)
        (set `PlayerController.bShowMouseCursor` true _returnvalue))
      (:`NewEnumerator1`
        (set `self.DebugMode_AttributeSet` "NewEnumerator2")
        (bind _attributesetpanel (`self.AttributeSetPanel`)
          (:`then`
            (bind _userbasecanvas_2 (message `/Game/BA_Rougelike/Blueprints/BPI/BPI_PlayerController.Get_BaseCanvas` (`self.GetController`)))
            (`/Game/BA_Rougelike/Blueprints/UMG/WBP_UserBaseCanvas.RemoveWidget` _userbasecanvas_2 _attributesetpanel)
            (set `PlayerController.bShowMouseCursor` false _returnvalue))
          (:`else`))))))

(event `EnhancedInput|/Game/BA_Rougelike/Input/Actions/IA_Debug_ShowTargetSystemRadius`
  (params (ActionValue :type Boolean) (ElapsedSeconds :type "Float (double-precision)") (TriggeredSeconds :type "Float (double-precision)") (InputAction :type "InputAction Object Reference" :default "/Game/BA_Rougelike/Input/Actions/IA_Debug_ShowTargetSystemRadius.IA_Debug_ShowTargetSystemRadius"))
  ;[1 1 1] 目标检测调试
  (:`Triggered`
    (switch `/Game/BA_Rougelike/GameData/Enums/Character/Debug/E_DebugMode` (`self.DebugMode_TargetSystem`)
      (:`NewEnumerator2`
        (set `self.DebugMode_TargetSystem` "NewEnumerator1"))
      (:`NewEnumerator1`
        (set `self.DebugMode_TargetSystem` "NewEnumerator2")))))

(event `self.ReceiveAnyDamage`
  (params (Damage :type "Float (single-precision)") (DamageType :type "DamageType Object Reference") (InstigatedBy :type "Controller Object Reference") (DamageCauser :type "Actor Object Reference"))
  (bind _damageout (message `/Game/BA_Rougelike/Blueprints/BPI/BPI_DamageType.ProcessDamage` DamageType Damage self InstigatedBy))
  ;[1 1 1] 动态伤害GE
  (bind _returnvalue (`AbilitySystemBlueprintLibrary.AssignTagSetByCallerMagnitude` (`AbilitySystemComponent.MakeOutgoingSpec` :`self` (`self.EnhancedInputAbilitySystem`) :`GameplayEffectClass` "/Game/BA_Rougelike/Blueprints/GAS/GE/GE_CommonDamage.GE_CommonDamage_C") (struct :`TagName` "AttributeData.Enemy.AttackDamage") (* _damageout -1.0)))
  (`AbilitySystemComponent.BP_ApplyGameplayEffectSpecToSelf` (`self.EnhancedInputAbilitySystem`) _returnvalue))

(event `/Game/BA_Rougelike/Blueprints/BPI/BPI_PlayerCharacter.Set_RotateMode`
  (params (RotateMode :type "/Game/BA_Rougelike/GameData/Enums/Character/Movement/E_CharacterRotateMode Enum" :default "NewEnumerator0"))
  ;[1 1 1] 转向控制
  (if (`|EnumInequality` RotateMode (`self.CurRotateMode`))
    (set `self.CurRotateMode` RotateMode)
    (set `self.bUseControllerRotationYaw` (select `/Game/BA_Rougelike/GameData/Enums/Character/Movement/E_CharacterRotateMode` (`self.CurRotateMode`) :`NewEnumerator1` true))
    (set `CharacterMovementComponent.bOrientRotationToMovement` (select `/Game/BA_Rougelike/GameData/Enums/Character/Movement/E_CharacterRotateMode` (`self.CurRotateMode`) :`NewEnumerator0` true) (`self.CharacterMovement`))))

(event `/Game/BA_Rougelike/Blueprints/BPI/BPI_PlayerCharacter.Set_NotAllowSwitchTarget`
  (params (NotAllowSwitchTarget :type Boolean))
  ;[1 1 1] 设置 是否可以切换目标
  (set `self.NotAllowSwitchTarget` NotAllowSwitchTarget))

(event `/Game/BA_Rougelike/Blueprints/BPI/BPI_CharacterCommon.Set_Group`
  (params (NewGroup :type "/Game/BA_Rougelike/GameData/Enums/E_ActorGroup Enum" :default "NewEnumerator0"))
  ;[1 1 1] 角色组覆写
  (set `self.Group` NewGroup))

(fn `BindAttributeChangeFun`
  (add `self.MoveSpeedChangedEvent` (`|CreateDelegate` :!event `OnMoveSpeedChanged`)))

(fn `ClearCurTarget`
  (message `/Game/BA_Rougelike/Blueprints/BPI/BPI_PlayerController.Clear_CurrentTarget` (`self.GetController`)))

(fn `Debug_TargetSystem`
  (`|ExecutionSequence`
    (:`then_0`
      (if (`|EnumEquality` (`self.DebugMode_TargetSystem`) "NewEnumerator1")
        (bind _range (`self.GetAttackRange`)
          (:`true`
            (`KismetSystemLibrary.DrawDebugCircle` (`self.K2_GetActorLocation`) _range 36 (struct :`G` 0.286018 :`B` 1.0 :`A` 1.0) 0.0 2.0 (0.0 1.0 0.0) (1.0 0.0 0.0))
            (bind _curtarget (message `/Game/BA_Rougelike/Blueprints/BPI/BPI_PlayerController.Get_CurrentTarget` (`self.GetController`)))
            (`/Engine/EditorBlueprintResources/StandardMacros.IsValid` _curtarget
              (:`Is Valid`
                (`KismetSystemLibrary.DrawDebugArrow` (`self.K2_GetActorLocation`) (`self.K2_GetActorLocation` _curtarget) 10.0 (struct :`G` 1.0 :`B` 0.077964 :`A` 1.0) 0.0 2.0)))))))))

(fn `EndLoopCheckTarget`
  (`KismetSystemLibrary.K2_ClearAndInvalidateTimerHandle` (`self.LoopCheckTargetTimer`)))

(fn `EndLoopWaitAttack`
  ;[1 1 1] 停止蒙太奇
  (`self.StopAnimMontage` (`self.AttackMontage`))
  ;[1 1 1] 结束等待攻击定时器
  (`KismetSystemLibrary.K2_ClearAndInvalidateTimerHandle` (`self.WaitForAttackHandel`))
  ;[1 1 1] 停止播放开火音效
  (`AudioComponent.FadeOut` (`self.AttackSoundComp`) 0.15 0.0 "Linear")
  (set `self.IsAlreadyAttacking` false))

(fn `Get_ArmorType`
  (returns (ArmorType :type "/Game/BA_Rougelike/GameData/Enums/E_ArmorType Enum"))
  (return (`self.ArmorType`)))

(fn `Get_AttackMontage`
  (returns (Montage :type "AnimMontage Object Reference"))
  (return (`self.AttackMontage`)))

(fn `Get_AttackType`
  (returns (AttackType :type "/Game/BA_Rougelike/GameData/Enums/E_AttackType Enum"))
  (return (`self.AttackType`)))

(fn `Get_Damage`
  (returns (Damage :type "Float (double-precision)"))
  (bind (_bsuccessfullyfoundattribute _returnvalue) (`AbilitySystemBlueprintLibrary.GetFloatAttribute` self (struct :`AttributeName` "AttackDamage" :`Attribute` "/Script/BA_Rougelike.MyAttributeSet_Character:AttackDamage" :`AttributeOwner` "/Script/CoreUObject.Class'/Script/BA_Rougelike.MyAttributeSet_Character'")))
  (if _bsuccessfullyfoundattribute
    (return _returnvalue)
    (else
      (return 0.0))))

(fn `Get_Group`
  (returns (Group :type "/Game/BA_Rougelike/GameData/Enums/E_ActorGroup Enum"))
  (return (`self.Group`)))

(fn `Get_HeadImage`
  (returns (HeadImage :type "Texture2D Object Reference"))
  (return (`self.HeadImage`)))

(fn `Get_Health`
  (returns (CurHealth :type "Float (double-precision)") (MaxHealth :type "Float (double-precision)"))
  (bind (_bsuccessfullyfoundattribute _returnvalue) (`AbilitySystemBlueprintLibrary.GetFloatAttribute` self (struct :`AttributeName` "MaxHealth" :`Attribute` "/Script/BA_Rougelike.MyAttributeSet_Character:MaxHealth" :`AttributeOwner` "/Script/CoreUObject.Class'/Script/BA_Rougelike.MyAttributeSet_Character'")))
  (bind (_bsuccessfullyfoundattribute_2 _returnvalue_2) (`AbilitySystemBlueprintLibrary.GetFloatAttribute` self (struct :`AttributeName` "Health" :`Attribute` "/Script/BA_Rougelike.MyAttributeSet_Character:Health" :`AttributeOwner` "/Script/CoreUObject.Class'/Script/BA_Rougelike.MyAttributeSet_Character'")))
  (if (and _bsuccessfullyfoundattribute_2 _bsuccessfullyfoundattribute)
    (return _returnvalue_2 _returnvalue)
    (else
      (return 0.0 0.0))))

(fn `Get_MoveSpeed`
  (returns (MoveSpeed :type "Float (double-precision)"))
  (bind (_bsuccessfullyfoundattribute _returnvalue) (`AbilitySystemBlueprintLibrary.GetFloatAttribute` self (struct :`AttributeName` "MoveSpeed" :`Attribute` "/Script/BA_Rougelike.MyAttributeSet_Character:MoveSpeed" :`AttributeOwner` "/Script/CoreUObject.Class'/Script/BA_Rougelike.MyAttributeSet_Character'")))
  (if _bsuccessfullyfoundattribute
    (return _returnvalue)
    (else
      (return 0.0))))

(fn `GetCurTarget`
  (returns (CurTarget :type "Actor Object Reference"))
  (bind _curtarget (message `/Game/BA_Rougelike/Blueprints/BPI/BPI_PlayerController.Get_CurrentTarget` (`self.GetController`)))
  (return _curtarget))

(fn `GetMontagePlatRate`
  (returns (ReturnValue :type "Float (double-precision)"))
  (bind (_bsuccessfullyfoundattribute _returnvalue) (`AbilitySystemBlueprintLibrary.GetFloatAttribute` self (struct :`AttributeName` "AttackSpeedMultiplier" :`Attribute` "/Script/BA_Rougelike.MyAttributeSet_Character:AttackSpeedMultiplier" :`AttributeOwner` "/Script/CoreUObject.Class'/Script/BA_Rougelike.MyAttributeSet_Character'")))
  (if _bsuccessfullyfoundattribute
    (return _returnvalue)
    (else
      (return 1.0))))

(fn `GetNearestTarget`
  (returns (NearestTarget :type "Actor Object Reference"))
  (locals (LocalMinDistance :type "Float (single-precision)" :default 0.0) (LocalCurTarget :type "Actor Object Reference"))
  (`self.IsAllowSwitchTarget` ; 当前是否允许切换
    (:`true`
      ;[1 1 1] 重置本地参数
      (set `local.LocalMinDistance` 99999.0)
      (set `local.LocalCurTarget` null)
      (for _array_element (`self.TargetList`)
        (bind _returnvalue (`self.GetDistanceTo` _array_element))
        ;[1 1 1] 找出最近目标
        (if (< _returnvalue (`local.LocalMinDistance`))
          (set `local.LocalMinDistance` _returnvalue)
          (set `local.LocalCurTarget` _array_element)))
      ;[1 1 1] 返回
      (return (`local.LocalCurTarget`)))
    (:`false`
      ;[1 1 1] 不允许切换 使用原来的目标
      (return (`self.GetCurTarget`)))))

(fn `InitAttackSound`
  (`AudioComponent.SetSound` (`self.AttackSoundComp`) (`self.AttackSoundCue`)))

(fn `InitBasicGAGE`
  (`|ExecutionSequence`
    (:`then_0`
      ;[1 1 1] 给予基础GA
      (bind _keys (`BlueprintMapLibrary.Map_Keys` (`self.BasicGA`)))
      (for _array_element _keys
        (bind (_ability _level) (break `/Game/BA_Rougelike/GameData/Structs/S_BasicGA` _array_element))
        (bind _returnvalue (`AbilitySystemComponent.K2_GiveAbility` (`self.EnhancedInputAbilitySystem`) _ability _level -1))
        (bind (_value _returnvalue_2) (`BlueprintMapLibrary.Map_Find` (`self.BasicGA`) _array_element))
        (if _returnvalue_2
          (`/Engine/EditorBlueprintResources/StandardMacros.IsValid` _value
            (:`Is Valid`
              (`EnhancedInputAbilitySystem.SetInputBinding` (`self.EnhancedInputAbilitySystem`) _value _returnvalue))))))
    (:`then_1`
      ;[1 1 1] 应用基础GE列表
      (bind _keys_2 (`BlueprintMapLibrary.Map_Keys` (`self.BasicGE`)))
      (for _array_element_2 _keys_2
        (bind (_value_2 _returnvalue_3) (`BlueprintMapLibrary.Map_Find` (`self.BasicGE`) _array_element_2))
        (if _returnvalue_3
          (`AbilitySystemComponent.BP_ApplyGameplayEffectToSelf` :`self` (`self.EnhancedInputAbilitySystem`) :`GameplayEffectClass` _array_element_2 :`Level` _value_2))))))

(fn `InitGroupMap`
  (`/Game/BA_Rougelike/Blueprints/SubSystem/BP_GroupSubsystem.RegisterToMap` (subsystem `/Game/BA_Rougelike/Blueprints/SubSystem/BP_GroupSubsystem`) self))

(fn `InitMappingContext`
  (bind `_as玩家控制器` (cast `PlayerController` (`self.GetController`)))
  (bind _returnvalue (pcsubsystem `EnhancedInputLocalPlayerSubsystem` `_as玩家控制器`))
  (`/Engine/EditorBlueprintResources/StandardMacros.IsValid` _returnvalue
    (:`Is Valid`
      (`EnhancedInputSubsystemInterface.AddMappingContext` _returnvalue "/Game/BA_Rougelike/Input/IMC_MyDefault.IMC_MyDefault" 0 (struct)))))

(fn `InitMoveSpeed`
  (bind (_bsuccessfullyfoundattribute _returnvalue) (`AbilitySystemBlueprintLibrary.GetFloatAttribute` self (struct :`AttributeName` "MoveSpeed" :`Attribute` "/Script/BA_Rougelike.MyAttributeSet_Character:MoveSpeed" :`AttributeOwner` "/Script/CoreUObject.Class'/Script/BA_Rougelike.MyAttributeSet_Character'")))
  (if _bsuccessfullyfoundattribute
    (set `CharacterMovementComponent.MaxWalkSpeed` _returnvalue (`self.CharacterMovement`))))

(fn `LoopCheckTarget`
  (locals (LocalOverlapActors :type "Array of Actor Object Reference") (LocalNearestTarget :type "Actor Object Reference"))
  ;[1 1 1] 范围Actor检测
  (bind _actorlist (`/Game/BA_Rougelike/Blueprints/SubSystem/BP_GroupSubsystem.GetSameGroupActorList` (subsystem `/Game/BA_Rougelike/Blueprints/SubSystem/BP_GroupSubsystem`) self))
  (bind _range (`self.GetAttackRange`)
    (:`true`
      (bind (_outactors _returnvalue) (`KismetSystemLibrary.SphereOverlapActors` (`self.K2_GetActorLocation`) _range (`|MakeArray` "ObjectTypeQuery3" :!type "EObjectTypeQuery Enum") null _actorlist))
      (if _returnvalue
        (set `local.LocalOverlapActors` _outactors)
        ;[1 1 1] 清空目标列表
        (`KismetArrayLibrary.Array_Clear` (`self.TargetList`))
        (for _array_element (`local.LocalOverlapActors`)
          (`self.IsTarget` _array_element ; 角色组是否为敌人
            (:`true`
              (`self.IsTargetAlive` _array_element ; 敌人是否存活
                (:`true`
                  ;[1 1 1] 添加到目标列表
                  (`KismetArrayLibrary.Array_Add` (`self.TargetList`) _array_element))))))
        (`self.IsTargetListEmpty` ; 目标列表是否为空
          (:`true`
            ;[1 1 1] 结束朝向与攻击
            (`self.ClearCurTarget` :!label _label) ; 清除玩家控制器当前目标
            (`self.EndLoopWaitAttack`) ; 结束循环攻击
          )
          (:`false`
            ;[0.6875 0.02164 0] 目标计算与攻击
            (`|ExecutionSequence`
              (:`then_0`
                ;;[1 1 1] 获取最近的目标
                (bind _nearesttarget (`self.GetNearestTarget`))
                (set `local.LocalNearestTarget` _nearesttarget))
              (:`then_1`
                ;;[1 1 1] 更新控制器当前目标
                ;;;[1 1 1] 当前的目标是否发生了切换？
                (if (!= (`self.GetCurTarget`) (`local.LocalNearestTarget`))
                  (`self.SetCurTarget` (`local.LocalNearestTarget`))))
              (:`then_2`
                ;;[1 1 1] 开始循环攻击
                (`self.StartLoopWaitAttack`)))))
        (else
          (goto _label))))))

(fn `OnMoveSpeedChanged`
  (params (OldValue :type "Float (double-precision)") (NewValue :type "Float (double-precision)"))
  (set `CharacterMovementComponent.MaxWalkSpeed` NewValue (`self.CharacterMovement`)))

(fn `SetCurTarget`
  (params (TargetActor :type "Actor Object Reference"))
  (message `/Game/BA_Rougelike/Blueprints/BPI/BPI_PlayerController.Set_CurrentTarget` (`self.GetController`) TargetActor))

(fn `StartLoopCheckTarget`
  (bind _returnvalue (`KismetSystemLibrary.K2_SetTimer` null "LoopCheckTarget" 0.1 true))
  (set `self.LoopCheckTargetTimer` _returnvalue))

(fn `StartLoopWaitAttack`
  ;[1 1 1] 从非战斗切换到战斗才触发
  (if (not (`self.IsAlreadyAttacking`))
    ;[1 1 1] 循环等待播放攻击蒙太奇
    (if (not (`KismetSystemLibrary.K2_IsTimerActiveHandle` (`self.WaitForAttackHandel`)))
      (bind _returnvalue (`KismetSystemLibrary.K2_SetTimer` null "WaitAttack" 0.1 true))
      (set `self.WaitForAttackHandel` _returnvalue))))

(fn `UserConstructionScript`
  (`self.InitAttackSound`)
  (`self.InitMoveSpeed`))

(fn `WaitAttack`
  ;[1 1 1] 是否已经面向目标
  (bind _curtarget (message `/Game/BA_Rougelike/Blueprints/BPI/BPI_PlayerController.Get_CurrentTarget` (`self.GetController`)))
  (`/Engine/EditorBlueprintResources/StandardMacros.IsValid` _curtarget
    (:`Is Valid`
      (if (`KismetMathLibrary.InRange_FloatFloat` (`KismetMathLibrary.Dot_VectorVector` (`KismetMathLibrary.GetForwardVector` (`self.K2_GetActorRotation` _curtarget)) (`KismetMathLibrary.GetForwardVector` (`self.K2_GetActorRotation`))) -1.0 -0.9)
        ;[1 1 1] 循环开火蒙太奇
        (`self.PlayAnimMontage` (`self.AttackMontage`) (`self.GetMontagePlatRate`))
        (set `self.IsAlreadyAttacking` true)
        ;;[1 1 1] 结束等待攻击定时器
        (`KismetSystemLibrary.K2_ClearAndInvalidateTimerHandle` (`self.WaitForAttackHandel`))
        ;[1 1 1] 设置开火音效组件音高
        (`AudioComponent.SetPitchMultiplier` (`self.AttackSoundComp`) (`self.GetMontagePlatRate`))
        ;[1 1 1] 播放开火音效
        (`AudioComponent.FadeIn` (`self.AttackSoundComp`) 0.1 1.0 0.0 "Linear")))))