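; Enemy spawner for a roguelike that runs wave countdowns from a data table keyed by wave index.
; After player setup, it pushes a wave info widget and updates it from a one-second timer, advancing the wave at zero.
; Spawn functions run an EQS query around the player and spawn enemies at random result locations with debug spheres.
; The sub-wave loop that schedules those queries is unconnected, so only countdowns run.
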(event `self.ReceiveBeginPlay`
  (set `self.CurWaveIndex` 1)
  (bind _asbp_my_character_base (cast `/Game/BA_Rougelike/Characters/BP_MyCharacter_Base` (`GameplayStatics.GetPlayerPawn` 0)))
  (add `/Game/BA_Rougelike/Characters/BP_MyCharacter_Base.OnBeginPlayComplete` _asbp_my_character_base (delegate `自定义事件`)))

(event `自定义事件`
  (bind _userbasecanvas (message `/Game/BA_Rougelike/GameData/BPI/BPI_PlayerCharacter.Get_BaseCanvas` (`GameplayStatics.GetPlayerPawn` 0)))
  (`/Engine/EditorBlueprintResources/StandardMacros.IsValid` _userbasecanvas
    (:`Is Valid`
      (bind _returnvalue (`/Game/BA_Rougelike/Blueprints/UMG/WBP_UserBaseCanvas.PushWidget` _userbasecanvas "/Game/BA_Rougelike/Blueprints/UMG/WBP_WaveInfo.WBP_WaveInfo_C"))
      (set `self.WaveWidget` _returnvalue)
      (`self.StartCountdown`))))

(event `StartCountdown`
  (bind _wavewidget (`self.WaveWidget`)
    (:`then`
      (message `/Game/BA_Rougelike/GameData/BPI/BPI_WaveWidget.UpdateWaveIndex` _wavewidget (`self.CurWaveIndex`))
      (bind _countdown (`self.GetCurWaveInfo`)
        (:`Success`
          (set `self.CurCountdownTime` _countdown)
          (`KismetSystemLibrary.K2_ClearAndInvalidateTimerHandle` (`self.CountdownHandel`))
          (bind _returnvalue (`KismetSystemLibrary.K2_SetTimerDelegate` (delegate `LoopCountDown`) 1.0 true))
          (set `self.CountdownHandel` _returnvalue))))
    (:`else`)))

(event `LoopCountDown`
  (`|ExecutionSequence`
    (:`then_0`
      (bind _result (`/Engine/EditorBlueprintResources/StandardMacros.DecrementInt` (`self.CurCountdownTime`))
        (:`  `
          (if (== _result 0)
            (`KismetSystemLibrary.K2_ClearAndInvalidateTimerHandle` (`self.CountdownHandel`))
            (`/Engine/EditorBlueprintResources/StandardMacros.IncrementInt` (`self.CurWaveIndex`)
              (:`  `
                (`self.StartCountdown`)))))))
    (:`then_1`
      (bind _wavewidget (`self.WaveWidget`)
        (:`then`
          (message `/Game/BA_Rougelike/GameData/BPI/BPI_WaveWidget.UpdateCountDown` _wavewidget (`self.CurCountdownTime`)))
        (:`else`)))))

(fn `GetCurWaveAsName`
  (returns (ReturnValue :type Name))
  (return (`KismetStringLibrary.Conv_StringToName` (`KismetStringLibrary.Conv_IntToString` (`self.CurWaveIndex`)))))

(fn `OnEQSQueryFinished`
  (params (QueryInstance :type "EnvQueryInstanceBlueprintWrapper Object Reference") (QueryStatus :type "EEnvQueryStatus Enum" :default "Processing"))
  (locals (Loc :type "Vector Structure"))
  (bind (_resultlocations _returnvalue) (`EnvQueryInstanceBlueprintWrapper.GetQueryResultsAsLocations` QueryInstance))
  (if _returnvalue
    (for _ (range (+ (`KismetMathLibrary.Min` (`KismetArrayLibrary.Array_Length` _resultlocations) (`.SpawnNum_9_A119D03942ED010821A457BA7566773A` (break `/Game/BA_Rougelike/GameData/Structs/S_SubWaveInfo` (`self.CurWaveSubInfo`)))) 1))
      (bind _output_get (set `local.Loc` (`KismetArrayLibrary.Array_Random` _resultlocations)))
      (`KismetSystemLibrary.DrawDebugSphere` _output_get 80.0 12 (struct :`R` 1.0 :`B` 0.003362 :`A` 1.0) 1.0 5.0)
      (`|SpawnActorFromClass` (`.SpawnActorClass_6_B4A9A15F45E58F6D6C863EA6C6EEE4C5` (break `/Game/BA_Rougelike/GameData/Structs/S_SubWaveInfo` (`self.CurWaveSubInfo`))) (`KismetMathLibrary.MakeTransform` (`local.Loc`)) "AdjustIfPossibleButAlwaysSpawn" "MultiplyWithRoot" null null))
    (remove `EnvQueryInstanceBlueprintWrapper.OnQueryFinishedEvent` QueryInstance (`|CreateDelegate` :!event `OnEQSQueryFinished`))))

(fn `StartEQSQuery`
  (bind _returnvalue (`EnvQueryManager.RunEQSQuery` "/Game/BA_Rougelike/AI/EQS/EQS_Player.EQS_Player" (`GameplayStatics.GetPlayerPawn` 0) "AllMatching"))
  (add `EnvQueryInstanceBlueprintWrapper.OnQueryFinishedEvent` _returnvalue (`|CreateDelegate` :!event `OnEQSQueryFinished`)))

(fn `UserConstructionScript`)