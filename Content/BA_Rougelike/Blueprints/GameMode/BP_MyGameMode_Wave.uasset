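; Wave-based game mode for a roguelike that spawns enemy sub-waves around the player and drives the wave HUD.
; After player init, NextWave loads the wave's DataTable row and starts a one-second countdown timer.
; Sub-waves matching the elapsed time run an EQS query, then spawn pooled enemies with Niagara effects at random result points, scaling health and damage by wave multipliers.
; Nothing here advances the wave when the countdown ends.
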(event `self.ReceiveBeginPlay`
  (`parent.ReceiveBeginPlay`)
  ;[1 1 1] 等待玩家初始化完毕
  (bind _asbp_my_character_base (cast `/Game/BA_Rougelike/Blueprints/Characters/BP_MyCharacter_Base` (`GameplayStatics.GetPlayerPawn` 0)))
  (add `/Game/BA_Rougelike/Blueprints/Characters/BP_MyCharacter_Base.OnBeginPlayComplete` _asbp_my_character_base (`|CreateDelegate` :!event `OnPlayerBeginPlayComplete`)))

(fn `DamageEnhance`
  (params (Actor :type "Actor Object Reference"))
  (bind _damage (message `/Game/BA_Rougelike/Blueprints/BPI/BPI_CharacterCommon.Get_Damage` Actor))
  (message `/Game/BA_Rougelike/Blueprints/BPI/BPI_Enemy.Set_Damage` Actor (* _damage (`KismetMathLibrary.FMax` (`.DamageMultipler_26_E82E10344A7F425636B277B3EE957C74` (break `/Game/BA_Rougelike/GameData/Structs/S_WaveInfo` (`self.CurWaveInfo`)))))))

(fn `GetCurWaveAsName`
  (returns (ReturnValue :type Name))
  (return (`KismetStringLibrary.Conv_StringToName` (`KismetStringLibrary.Conv_IntToString` (`self.CurWaveIndex`)))))

(fn `GetWaveWidget`
  (bind _waveinfo (message `/Game/BA_Rougelike/Blueprints/BPI/BPI_PlayerController.Get_HUD_WaveInfo` (`GameplayStatics.GetPlayerController` 0)))
  (set `self.WaveInfoWidget` _waveinfo)
  (`self.GetCurWaveInfo`
    (:`Success`
      (message `/Game/BA_Rougelike/Blueprints/BPI/BPI_WaveWidget.UpdateCountDown` (`self.WaveInfoWidget`) 0))))

(fn `HealthEnhance`
  (params (Actor :type "Actor Object Reference"))
  (bind (_curhealth _maxhealth) (message `/Game/BA_Rougelike/Blueprints/BPI/BPI_CharacterCommon.Get_Health` Actor))
  (bind _returnvalue (* _maxhealth (`KismetMathLibrary.FMax` (`.HealthMultipler_24_19AD761A4DFCDD6AF2D3BCB09D6DB93E` (break `/Game/BA_Rougelike/GameData/Structs/S_WaveInfo` (`self.CurWaveInfo`))))))
  (message `/Game/BA_Rougelike/Blueprints/BPI/BPI_Enemy.Set_Health` Actor _returnvalue _returnvalue))

(fn `LoopCurWave`
  (locals (LocalFindSubWave :type Boolean) (LocalSubWaveInfo :type "/Game/BA_Rougelike/GameData/Structs/S_SubWaveInfo Structure") (LocalSubWaveIndex :type Integer))
  (`|ExecutionSequence`
    (:`then_0`
      ;[1 1 1] 当前主波次倒计时自减 为0时清除当前主波次定时器
      (bind _result (`/Engine/EditorBlueprintResources/StandardMacros.DecrementInt` (`self.CurWaveCountdown`)) ; 倒计时自减
        (:`  `
          (if (== _result 0)
            (`KismetSystemLibrary.K2_ClearAndInvalidateTimerHandle` (`self.CurWaveTimer`))))))
    (:`then_1`
      ;[1 1 1] 更新当前主波次倒计时UMG
      (bind _waveinfowidget (`self.WaveInfoWidget`)
        (:`then`
          (message `/Game/BA_Rougelike/Blueprints/BPI/BPI_WaveWidget.UpdateCountDown` _waveinfowidget (`self.CurWaveCountdown`)))
        (:`else`)))
    (:`then_2`
      ;[1 1 1] 循环查询对应子波次的信息
      (bind _curwaveinfo (`self.GetCurWaveInfo`)
        (:`Success`
          (bind ((`Countdown_19_5FAE711745080ECEDFF7429674B90CFA` _countdown) (`SubWaveInfo_20_B8D27F7F40A4C797BDB00F90605C5C75` _subwaveinfo)) (break `/Game/BA_Rougelike/GameData/Structs/S_WaveInfo` _curwaveinfo))
          (for (_array_element _array_index) _subwaveinfo
            (if (== (`.SpawnTimeAtCurWave_14_0A3AE45441C26C61157B06B02B543FF3` (break `/Game/BA_Rougelike/GameData/Structs/S_SubWaveInfo` _array_element)) (- _countdown (`self.CurWaveCountdown`)))
              (set `local.LocalFindSubWave` true)
              (set `local.LocalSubWaveInfo` _array_element)
              (set `local.LocalSubWaveIndex` _array_index)
              (break)
              (else
                (set `local.LocalFindSubWave` false))))
          (if (`local.LocalFindSubWave`)
            (`|ExecutionSequence`
              (:`then_0`
                ;[1 1 1] 更新子波次信息和索引
                (set `self.SubWaveInfo` (`local.LocalSubWaveInfo`))
                (set `self.CurSubWaveIndex` (`local.LocalSubWaveIndex`)))
              (:`then_1`
                ;[1 1 1] 更新子波次计数UMG
                (message `/Game/BA_Rougelike/Blueprints/BPI/BPI_WaveWidget.UpdateSubWaveIndex` (`self.WaveInfoWidget`) (`self.CurSubWaveIndex`)))
              (:`then_2`
                ;[1 1 1] 开始EQS查询生成敌人
                (`self.StartEQSQuery`)))))))))

(fn `NextWave`
  (`|ExecutionSequence`
    (:`then_0`
      ;[1 1 1] 主波次索引自增（默认为0）
      (`/Engine/EditorBlueprintResources/StandardMacros.IncrementInt` (`self.CurWaveIndex`)))
    (:`then_1`
      ;[1 1 1] 更新主波次计数UMG
      (bind _waveinfowidget (`self.WaveInfoWidget`)
        (:`then`
          (message `/Game/BA_Rougelike/Blueprints/BPI/BPI_WaveWidget.UpdateWaveIndex` _waveinfowidget (`self.CurWaveIndex`)) ; 更新一次波次索引
        )
        (:`else`)))
    (:`then_2`
      ;[1 1 1] 当前主波次信息和倒计时秒数
      (bind _curwaveinfo (`self.GetCurWaveInfo`)
        (:`Success`
          (set `self.CurWaveInfo` _curwaveinfo)
          (set `self.CurWaveCountdown` (`.Countdown_19_5FAE711745080ECEDFF7429674B90CFA` (break `/Game/BA_Rougelike/GameData/Structs/S_WaveInfo` _curwaveinfo))))))
    (:`then_3`
      ;[1 1 1] 开始当前波次倒计时
      (`self.StartLoopCurWave`))))

(fn `OnEQSQueryFinished`
  (params (QueryInstance :type "EnvQueryInstanceBlueprintWrapper Object Reference") (QueryStatus :type "EEnvQueryStatus Enum" :default "Processing"))
  (locals (SpawnLoc :type "Vector Structure") (LocalResultLocations :type "Array of Vector Structure") (LocalSpawnedActor :type "Actor Object Reference"))
  ;[1 1 1] 子波次敌人生成逻辑
  (bind (_resultlocations _returnvalue) (`EnvQueryInstanceBlueprintWrapper.GetQueryResultsAsLocations` QueryInstance))
  (bind _output_get (set `local.LocalResultLocations` _resultlocations))
  (bind _returnvalue_2 (`self.GetSpawnNum` _output_get _returnvalue) ; 获取生成数量
    (:`true`
      (for _ (range 1 (+ _returnvalue_2 1))
        (bind _output_get_2 (set `local.SpawnLoc` (`KismetArrayLibrary.Array_Random` (`local.LocalResultLocations`))))
        (`self.SapwnFX` _output_get_2) ; 生成特效
        (bind _spawnedactor (`self.SpawnActor` (`local.SpawnLoc`))) ; 生成Actor
        (set `local.LocalSpawnedActor` _spawnedactor)
        ;[1 1 1] 生命值与伤害增强
        (`self.HealthEnhance` (`local.LocalSpawnedActor`))
        (`self.DamageEnhance` (`local.LocalSpawnedActor`)))
      ;[1 1 1] 事件解绑
      (remove `EnvQueryInstanceBlueprintWrapper.OnQueryFinishedEvent` (`local.QueryInstance`) (`|CreateDelegate` :!event `OnEQSQueryFinished`)))))

(fn `OnPlayerBeginPlayComplete`
  (`self.GetWaveWidget`) ; 添加波次信息UMG
  (`self.NextWave`) ; 开始当前波次倒计时
)

(fn `SapwnFX`
  (params (Loc :type "Vector Structure"))
  (`NiagaraFunctionLibrary.SpawnSystemAtLocation` "/Game/BA_Rougelike/Niagara/NS_EnemySpawn.NS_EnemySpawn" Loc (struct) (1.0 1.0 1.0) true true "AutoRelease"))

(fn `SpawnActor`
  (params (Location :type "Vector Structure"))
  (returns (SpawnedActor :type "Actor Object Reference"))
  ;[1 1 1] 一律从对象池生成
  (bind _spawnedactor (`PoolSubsystem.SpawnFromPool` :`self` (subsystem `PoolSubsystem`) :`PoolClass` (`.SpawnActorClass_6_B4A9A15F45E58F6D6C863EA6C6EEE4C5` (break `/Game/BA_Rougelike/GameData/Structs/S_SubWaveInfo` (`self.SubWaveInfo`))) :`Location` (`local.Location`)))
  (return _spawnedactor))

(fn `StartEQSQuery`
  (bind _returnvalue (`EnvQueryManager.RunEQSQuery` "/Game/BA_Rougelike/Blueprints/AI/EQS/EQS_Player.EQS_Player" (`GameplayStatics.GetPlayerPawn` 0) "AllMatching"))
  (add `EnvQueryInstanceBlueprintWrapper.OnQueryFinishedEvent` _returnvalue (`|CreateDelegate` :!event `OnEQSQueryFinished`)))

(fn `StartLoopCurWave`
  ;[1 1 1] 当前波次倒计时
  (`KismetSystemLibrary.K2_ClearAndInvalidateTimerHandle` (`self.CurWaveTimer`))
  (bind _returnvalue (`KismetSystemLibrary.K2_SetTimer` null "LoopCurWave" 1.0 true))
  (set `self.CurWaveTimer` _returnvalue))

(fn `UserConstructionScript`
  (`parent.UserConstructionScript`))