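; Character component that tracks the player's team and drives the HUD team panel, which has four member slots.
; Once the owner finishes BeginPlay, it stores the player character in the list, fetches the team widget and fills or collapses each slot.
; Filled slots show portrait, health, EXP and level from float attributes.
; Attribute-change delegates route to callbacks that refresh the widget by member index, with a matching unbind event.
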(event `self.ReceiveBeginPlay`
  ;[1 1 1] 初始化
  (bind _asbp_my_character_base (cast `/Game/BA_Rougelike/Blueprints/Characters/BP_MyCharacter_Base` (`self.GetOwner`)))
  (bind _output_get (set `self.OwnerCharacter` _asbp_my_character_base))
  (add `/Game/BA_Rougelike/Blueprints/Characters/BP_MyCharacter_Base.OnBeginPlayComplete` _output_get (`|CreateDelegate` :!event `OnPlayerBeginPlayComplete`)))

(event `BindMemberInfo`
  (params (Index :type Integer))
  ;[1 1 1] 将UI信息变更绑定到角色属性变化委托
  (bind _member (`self.GetTeamMember` Index)
    (:`Is Valid`
      (add `MyCharacterBase.HealthChangedEvent` _member (delegate `OnHealthChanged`))
      (add `MyCharacterBase.MaxHealthChangedEvent` _member (delegate `OnMaxHealthChanged`))
      (add `MyCharacterBase.EXPChangedEvent` _member (delegate `OnEXPChanged`))
      (add `MyCharacterBase.MaxEXPChangedEvent` _member (delegate `OnMaxExpChanged`))
      (add `MyCharacterBase.LevelChangedEvent` _member (delegate `OnLevelChanged`)))))

(event `OnHealthChanged`
  (params (OldValue :type "Float (single-precision)") (NewValue :type "Float (single-precision)"))
  ;[1 1 1] 将UI信息变更绑定到角色属性变化委托
  (`self.HealthChangeCallback` (stale `BindMemberInfo` Index) NewValue))

(event `OnMaxHealthChanged`
  (params (OldValue :type "Float (single-precision)") (NewValue :type "Float (single-precision)"))
  ;[1 1 1] 将UI信息变更绑定到角色属性变化委托
  (`self.MaxHealthChangeCallback` (stale `BindMemberInfo` Index) NewValue))

(event `OnEXPChanged`
  (params (OldValue :type "Float (single-precision)") (NewValue :type "Float (single-precision)"))
  ;[1 1 1] 将UI信息变更绑定到角色属性变化委托
  (`self.EXPChangeCallback` (stale `BindMemberInfo` Index) NewValue))

(event `OnMaxExpChanged`
  (params (OldValue :type "Float (single-precision)") (NewValue :type "Float (single-precision)"))
  ;[1 1 1] 将UI信息变更绑定到角色属性变化委托
  (`self.MaxEXPChangeCallback` (stale `BindMemberInfo` Index) NewValue))

(event `OnLevelChanged`
  (params (OldValue :type "Float (single-precision)") (NewValue :type "Float (single-precision)"))
  ;[1 1 1] 将UI信息变更绑定到角色属性变化委托
  (`self.LevelChangeCallback` (stale `BindMemberInfo` Index) (`KismetMathLibrary.FTrunc` NewValue)))

(event `UnbindMemberInfo`
  (params (Index :type Integer))
  ;[1 1 1] 解绑指定索引队友的所有UI变化事件绑定
  (bind _member (`self.GetTeamMember` Index)
    (:`Is Valid`
      (remove `MyCharacterBase.HealthChangedEvent` _member (delegate `OnHealthChanged`))
      (remove `MyCharacterBase.MaxHealthChangedEvent` _member (delegate `OnMaxHealthChanged`))
      (remove `MyCharacterBase.EXPChangedEvent` _member (delegate `OnEXPChanged`))
      (remove `MyCharacterBase.MaxEXPChangedEvent` _member (delegate `OnMaxExpChanged`))
      (remove `MyCharacterBase.LevelChangedEvent` _member (delegate `OnLevelChanged`)))))

(fn `AddPlayerToList`
  (returns (Success :type Boolean))
  (bind _asbp_my_character_base (cast `/Game/BA_Rougelike/Blueprints/Characters/BP_MyCharacter_Base` (`GameplayStatics.GetPlayerCharacter` 0))
    (:`then`
      (`KismetArrayLibrary.Array_Set` (`self.TeamMemberList`) 0 _asbp_my_character_base true)
      (return true))
    (:`CastFailed`
      (return false))))

(fn `EXPChangeCallback`
  (params (Index :type Integer) (curEXP :type "Float (double-precision)"))
  (locals (LocalIndex :type Integer))
  (bind _output_get (set `local.LocalIndex` Index))
  (bind _member (`self.GetTeamMember` _output_get)
    (:`Is Valid`
      (bind (_bsuccessfullyfoundattribute _returnvalue) (`AbilitySystemBlueprintLibrary.GetFloatAttribute` _member (struct :`AttributeName` "MaxEXP" :`Attribute` "/Script/BA_Rougelike.MyAttributeSet_Character:MaxEXP" :`AttributeOwner` "/Script/CoreUObject.Class'/Script/BA_Rougelike.MyAttributeSet_Character'")))
      (if _bsuccessfullyfoundattribute
        (bind _returnvalue_2 (`self.GetMebmberWidget` (`local.LocalIndex`)))
        (`/Game/BA_Rougelike/Blueprints/UMG/WBP_PlayerInfoUnit.UpdateEXP` _returnvalue_2 (`local.curEXP`) _returnvalue)))))

(fn `GetTeamWidget`
  (bind _teaminfo (message `/Game/BA_Rougelike/Blueprints/BPI/BPI_PlayerController.Get_HUD_TeamInfo` (`GameplayStatics.GetPlayerController` 0)))
  (set `self.TeamInfoWidget` _teaminfo))

(fn `HealthChangeCallback`
  (params (Index :type Integer) (CurHealth :type "Float (double-precision)"))
  (locals (LocalIndex :type Integer))
  (bind _output_get (set `local.LocalIndex` Index))
  (bind _member (`self.GetTeamMember` _output_get)
    (:`Is Valid`
      (bind (_bsuccessfullyfoundattribute _returnvalue) (`AbilitySystemBlueprintLibrary.GetFloatAttribute` _member (struct :`AttributeName` "MaxHealth" :`Attribute` "/Script/BA_Rougelike.MyAttributeSet_Character:MaxHealth" :`AttributeOwner` "/Script/CoreUObject.Class'/Script/BA_Rougelike.MyAttributeSet_Character'")))
      (if _bsuccessfullyfoundattribute
        (bind _returnvalue_2 (`self.GetMebmberWidget` (`local.LocalIndex`)))
        (`/Game/BA_Rougelike/Blueprints/UMG/WBP_PlayerInfoUnit.UpdateHealth` _returnvalue_2 (`local.CurHealth`) _returnvalue)))))

(fn `InitMemberInfo`
  (params (Member :type "Actor Object Reference") (MemberInfoWidget :type "/Game/BA_Rougelike/Blueprints/UMG/WBP_PlayerInfoUnit Object Reference"))
  (bind _member (`local.Member`))
  (bind _member_2 (`local.Member`))
  (bind (_bsuccessfullyfoundattribute _returnvalue) (`AbilitySystemBlueprintLibrary.GetFloatAttribute` _member_2 (struct :`AttributeName` "MaxEXP" :`Attribute` "/Script/BA_Rougelike.MyAttributeSet_Character:MaxEXP" :`AttributeOwner` "/Script/CoreUObject.Class'/Script/BA_Rougelike.MyAttributeSet_Character'")))
  (bind (_bsuccessfullyfoundattribute_2 _returnvalue_2) (`AbilitySystemBlueprintLibrary.GetFloatAttribute` (`local.Member`) (struct :`AttributeName` "Level" :`Attribute` "/Script/BA_Rougelike.MyAttributeSet_Character:Level" :`AttributeOwner` "/Script/CoreUObject.Class'/Script/BA_Rougelike.MyAttributeSet_Character'")))
  (bind (_bsuccessfullyfoundattribute_3 _returnvalue_3) (`AbilitySystemBlueprintLibrary.GetFloatAttribute` _member (struct :`AttributeName` "Health" :`Attribute` "/Script/BA_Rougelike.MyAttributeSet_Character:Health" :`AttributeOwner` "/Script/CoreUObject.Class'/Script/BA_Rougelike.MyAttributeSet_Character'")))
  (bind (_bsuccessfullyfoundattribute_4 _returnvalue_4) (`AbilitySystemBlueprintLibrary.GetFloatAttribute` _member (struct :`AttributeName` "MaxHealth" :`Attribute` "/Script/BA_Rougelike.MyAttributeSet_Character:MaxHealth" :`AttributeOwner` "/Script/CoreUObject.Class'/Script/BA_Rougelike.MyAttributeSet_Character'")))
  (bind (_bsuccessfullyfoundattribute_5 _returnvalue_5) (`AbilitySystemBlueprintLibrary.GetFloatAttribute` _member_2 (struct :`AttributeName` "EXP" :`Attribute` "/Script/BA_Rougelike.MyAttributeSet_Character:EXP" :`AttributeOwner` "/Script/CoreUObject.Class'/Script/BA_Rougelike.MyAttributeSet_Character'")))
  (`|ExecutionSequence`
    (:`then_0`
      ;[1 1 1] 初始化血条
      (if (and _bsuccessfullyfoundattribute_3 _bsuccessfullyfoundattribute_4)
        (`/Game/BA_Rougelike/Blueprints/UMG/WBP_PlayerInfoUnit.UpdateHealth` (`local.MemberInfoWidget`) _returnvalue_3 _returnvalue_4)))
    (:`then_1`
      ;[1 1 1] 初始化经验条
      (if (and _bsuccessfullyfoundattribute_5 _bsuccessfullyfoundattribute)
        (`/Game/BA_Rougelike/Blueprints/UMG/WBP_PlayerInfoUnit.UpdateEXP` (`local.MemberInfoWidget`) _returnvalue_5 _returnvalue)))
    (:`then_2`
      ;[1 1 1] 初始化等级
      (if _bsuccessfullyfoundattribute_2
        (`/Game/BA_Rougelike/Blueprints/UMG/WBP_PlayerInfoUnit.UpdateLevel` (`local.MemberInfoWidget`) (`KismetMathLibrary.FTrunc` _returnvalue_2))))
    (:`then_3`
      ;[1 1 1] 初始化头像
      (bind _headimage (message `/Game/BA_Rougelike/Blueprints/BPI/BPI_PlayerCharacter.Get_HeadImage` (`local.Member`)))
      (`Image.SetBrushFromTexture` (`/Game/BA_Rougelike/Blueprints/UMG/WBP_PlayerInfoUnit.HeadImage` (`local.MemberInfoWidget`)) _headimage false))))

(fn `LevelChangeCallback`
  (params (Index :type Integer) (Level :type Integer))
  (locals (LocalIndex :type Integer))
  (bind _output_get (set `local.LocalIndex` Index))
  (bind _returnvalue (`self.GetMebmberWidget` _output_get))
  (`/Game/BA_Rougelike/Blueprints/UMG/WBP_PlayerInfoUnit.UpdateLevel` _returnvalue Level))

(fn `MaxEXPChangeCallback`
  (params (Index :type Integer) (maxEXP :type "Float (double-precision)"))
  (locals (LocalIndex :type Integer))
  (bind _output_get (set `local.LocalIndex` Index))
  (bind _member (`self.GetTeamMember` _output_get)
    (:`Is Valid`
      (bind (_bsuccessfullyfoundattribute _returnvalue) (`AbilitySystemBlueprintLibrary.GetFloatAttribute` _member (struct :`AttributeName` "EXP" :`Attribute` "/Script/BA_Rougelike.MyAttributeSet_Character:EXP" :`AttributeOwner` "/Script/CoreUObject.Class'/Script/BA_Rougelike.MyAttributeSet_Character'")))
      (if _bsuccessfullyfoundattribute
        (bind _returnvalue_2 (`self.GetMebmberWidget` (`local.LocalIndex`)))
        (`/Game/BA_Rougelike/Blueprints/UMG/WBP_PlayerInfoUnit.UpdateEXP` _returnvalue_2 _returnvalue (`local.maxEXP`))))))

(fn `MaxHealthChangeCallback`
  (params (Index :type Integer) (MaxHealth :type "Float (double-precision)"))
  (locals (LocalIndex :type Integer))
  (bind _output_get (set `local.LocalIndex` Index))
  (bind _member (`self.GetTeamMember` _output_get)
    (:`Is Valid`
      (bind (_bsuccessfullyfoundattribute _returnvalue) (`AbilitySystemBlueprintLibrary.GetFloatAttribute` _member (struct :`AttributeName` "Health" :`Attribute` "/Script/BA_Rougelike.MyAttributeSet_Character:Health" :`AttributeOwner` "/Script/CoreUObject.Class'/Script/BA_Rougelike.MyAttributeSet_Character'")))
      (if _bsuccessfullyfoundattribute
        (bind _returnvalue_2 (`self.GetMebmberWidget` (`local.LocalIndex`)))
        (`/Game/BA_Rougelike/Blueprints/UMG/WBP_PlayerInfoUnit.UpdateHealth` _returnvalue_2 _returnvalue (`local.MaxHealth`))))))

(fn `OnPlayerBeginPlayComplete`
  (bind _success (`self.AddPlayerToList`))
  (if _success
    (`self.GetTeamWidget`)
    (`self.UpdateTeamInfo`)))

(fn `UpdateTeamInfo`
  (locals (CurIndex :type Integer) (CurMemberWidget :type "/Game/BA_Rougelike/Blueprints/UMG/WBP_PlayerInfoUnit Object Reference"))
  (bind _curmemberwidget (`local.CurMemberWidget`))
  ;[1 1 1] 队友信息更新与绑定
  (for _index (range 4)
    ;;[1 1 1] 当前成员信息UI
    (bind _output_get (set `local.CurIndex` _index))
    (bind _returnvalue (`self.GetMebmberWidget` _output_get))
    (set `local.CurMemberWidget` _returnvalue)
    ;;[1 1 1] 控制可视性
    (bind _member (`self.GetTeamMember` (`local.CurIndex`))
      (:`Is Valid`
        (set `Widget.Visibility` "SelfHitTestInvisible" _curmemberwidget)
        (`self.InitMemberInfo` _member _curmemberwidget) ; 执行一次初始化
        ;[1 1 1] UMG绑定
        (`self.BindMemberInfo` (`local.CurIndex`)))
      (:`Is Not Valid`
        (set `Widget.Visibility` "Collapsed" _curmemberwidget)))))