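; Actor component that gives player and enemy characters a floating screen-space health bar, shown only briefly after health changes.
; On BeginPlay it binds to the owner's health event and builds a runtime widget component with WBP_Healthbar_New, waiting for player BeginPlay completion first.
; Fill color is green for the player group and armor-type based for others.
; Each update reveals the bar and restarts a timer that collapses it.
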(event `self.ReceiveBeginPlay`
  (bind `_as角色` (cast `Character` (`self.GetOwner`)))
  (bind _output_get (set `self.OwnerCharacter` `_as角色`))
  (bind _group (message `/Game/BA_Rougelike/Blueprints/BPI/BPI_CharacterCommon.Get_Group` _output_get))
  (switch `/Game/BA_Rougelike/GameData/Enums/E_ActorGroup` _group
    (:`NewEnumerator1`
      ;[1 1 1] 玩家/队友
      (bind _asbp_my_character_base (cast `/Game/BA_Rougelike/Blueprints/Characters/BP_MyCharacter_Base` (`self.OwnerCharacter`)))
      (add `/Game/BA_Rougelike/Blueprints/Characters/BP_MyCharacter_Base.OnBeginPlayComplete` _asbp_my_character_base (delegate `OnPlayerBeginPlayComplete`))
      (add `MyCharacterBase.HealthChangedEvent` _asbp_my_character_base (`|CreateDelegate` :!event `UpdateHealthBar`)))
    (:`NewEnumerator2`
      ;[1 1 1] 敌人
      (`self.InitializeHealthBar`)
      (bind _asbp_enemy_base (cast `/Game/BA_Rougelike/Blueprints/AI/Actors/Enemys/BP_Enemy_Base` (`self.OwnerCharacter`)))
      (add `/Game/BA_Rougelike/Blueprints/AI/Actors/Enemys/BP_Enemy_Base.CurHealthChanged` _asbp_enemy_base (`|CreateDelegate` :!event `UpdateHealthBar`)))))

(event `OnPlayerBeginPlayComplete`
  ;[1 1 1] 玩家/队友
  (`self.InitializeHealthBar`))

(fn `GetHealthBarColor`
  (returns (Value :type "LinearColor Structure"))
  (bind _group (message `/Game/BA_Rougelike/Blueprints/BPI/BPI_CharacterCommon.Get_Group` (`self.OwnerCharacter`)))
  (if (`|EnumEquality` _group "NewEnumerator1")
    (return (struct :`G` 0.697917 :`B` 0.002983 :`A` 1.0))
    (else
      (return (`/Game/BA_Rougelike/Blueprints/BFL/BFL_Common.GetArmorTypeColor` (`self.OwnerCharacter`))))))

(fn `HideHealthBar`
  (`self.SetHealthBarVisible` "Collapsed"))

(fn `InitializeHealthBar`
  (locals (LocalCueHealth :type "Float (double-precision)") (LocalMaxHealth :type "Float (double-precision)"))
  ;[1 1 1] 创建组件
  (bind _returnvalue (`|AddComponentByClass` (`self.OwnerCharacter`) "/Script/UMG.WidgetComponent" true (`self.Relative Transform`)))
  (set `self.WidgetComp` _returnvalue)
  (`WidgetComponent.SetWidgetSpace` (`self.WidgetComp`) "Screen") ; 设置为屏幕空间
  (`PrimitiveComponent.SetCollisionEnabled` (`self.WidgetComp`) "NoCollision") ; 关闭碰撞
  (`WidgetComponent.SetDrawAtDesiredSize` (`self.WidgetComp`) true) ; 按需绘制
  ;[1 1 1] 设置UMG对象
  (bind _returnvalue_2 (`|CreateWidget` "/Game/BA_Rougelike/Blueprints/UMG/WBP_Healthbar_New.WBP_Healthbar_New_C"))
  (bind _output_get (set `self.HealthBarWidgetObject` _returnvalue_2))
  (`WidgetComponent.SetWidget` (`self.WidgetComp`) _output_get)
  ;[1 1 1] 附加到拥有者的根组件
  (`SceneComponent.K2_AttachToComponent` (`self.WidgetComp`) (`Actor.RootComponent` (`self.GetOwner`)) "None" "KeepRelative" "KeepRelative" "KeepRelative" true)
  ;[1 1 1] 初始化血条颜色
  (`/Game/BA_Rougelike/Blueprints/UMG/WBP_Healthbar_New.InitializeFillColor` (`self.HealthBarWidgetObject`) (`self.GetHealthBarColor`))
  ;[1 1 1] 初始隐藏
  (`self.HideHealthBar`))

(fn `SetHealthBarVisible`
  (params (InVisibility :type "ESlateVisibility Enum" :default "Visible"))
  (`Widget.SetVisibility` (`self.HealthBarWidgetObject`) InVisibility))

(fn `UpdateHealthBar`
  (params (OldValue :type "Float (double-precision)") (NewValue :type "Float (double-precision)"))
  (bind (_curhealth _maxhealth) (message `/Game/BA_Rougelike/Blueprints/BPI/BPI_CharacterCommon.Get_Health` (`self.OwnerCharacter`)))
  (`self.SetHealthBarVisible` "SelfHitTestInvisible")
  (`/Game/BA_Rougelike/Blueprints/UMG/WBP_Healthbar_New.Health Changed` (`self.HealthBarWidgetObject`) (`local.OldValue`) (`local.NewValue`) _maxhealth)
  ;[1 1 1] 延迟隐藏
  (`KismetSystemLibrary.K2_ClearAndInvalidateTimerHandle` (`self.HideHealthBarTimer`))
  (bind _returnvalue (`KismetSystemLibrary.K2_SetTimer` null "HideHealthBar" (`self.HideDelayTime`)))
  (set `self.HideHealthBarTimer` _returnvalue))