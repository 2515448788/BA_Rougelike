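; Character component that finds the nearest interactable object around its owner and handles long-press interaction with it.
; Each tick, a sphere overlap keeps actors whose BPI_InteractiveObject info allows interaction and targets the closest.
; For player-controlled owners, a screen-projected WBP_InteractTip marks manual-interaction targets.
; IA_Interaction starts a looping timer for timed targets, filling the tip's progress and activating the target when its required time elapses.
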(event `self.ReceiveBeginPlay`
  (`self.GetOwnerCharacter`)
  (`self.IsPlayer` ; 是否为玩家
    (:`真`
      (bind _ownercharacter (`self.OwnerCharacter`)
        (:`then`
          (add `/Game/BA_Rougelike/Blueprints/Characters/BP_MyCharacter_Base.OnBeginPlayComplete` _ownercharacter (delegate `BeginPlayComplete`)))
        (:`else`)))))

(event `BeginPlayComplete`
  (`self.CreateInteractTip`))

(event `self.ReceiveTick`
  (params (DeltaSeconds :type "Float (single-precision)"))
  (`self.LoopCheckTarget`))

(event `EnhancedInput|/Game/BA_Rougelike/Input/Actions/IA_Interaction`
  (params (ActionValue :type Boolean) (ElapsedSeconds :type "Float (double-precision)") (TriggeredSeconds :type "Float (double-precision)") (InputAction :type "InputAction Object Reference" :default "/Game/BA_Rougelike/Input/Actions/IA_Interaction.IA_Interaction"))
  (:`Triggered`
    (`self.EndLongPressInteract`))
  (:`Started`
    (bind _currenttarget (`self.CurrentTarget`)
      (:`then`
        (`self.NeedLongPress` _currenttarget
          (:`真`
            (`self.StartLongPressInteract`))))
      (:`else`))))

(fn `CreateInteractTip`
  (bind _returnvalue (`|CreateWidget` "/Game/BA_Rougelike/Blueprints/UMG/WBP_InteractTip.WBP_InteractTip_C"))
  (bind _output_get (set `self.ItneractTipWidget` _returnvalue))
  (`UserWidget.AddToViewport` _output_get 0))

(fn `EndLongPressInteract`
  (`KismetSystemLibrary.K2_ClearAndInvalidateTimerHandle` (`self.LongPressInteractFun`))
  (set `self.CurInteractTime` 0.0)
  (`self.UpdateInteractProgess` 0.0)
  (`self.SetIconScale` 1.0))

(fn `GetCloestActor`
  (returns (Success :type Boolean) (Actor :type "Actor Object Reference"))
  (locals (Distance :type "Float (double-precision)" :default 0.0) (IsFind :type Boolean) (CloestActor :type "Actor Object Reference"))
  (bind _interactiveactorlist (`self.InteractiveActorList`))
  (set `local.Distance` 999999999.0)
  (set `local.IsFind` false)
  (if (`KismetArrayLibrary.Array_IsNotEmpty` _interactiveactorlist)
    (for _array_element _interactiveactorlist
      (bind _returnvalue (`Actor.GetDistanceTo` _array_element (`self.OwnerCharacter`)))
      (if (< _returnvalue (`local.Distance`))
        (set `local.Distance` _returnvalue)
        (set `local.CloestActor` _array_element)
        (set `local.IsFind` true)))
    ;[1 1 1] 返回
    (return (`local.IsFind`) (`local.CloestActor`))
    (else
      ;[1 1 1] 失败 返回
      (return false null))))

(fn `GetOwnerCharacter`
  (bind _asbp_my_character_base (cast `/Game/BA_Rougelike/Blueprints/Characters/BP_MyCharacter_Base` (`self.GetOwner`)))
  (set `self.OwnerCharacter` _asbp_my_character_base))

(fn `HideTip`
  (`self.OwnerIsPlayer` ; 仅玩家
    (:`then`
      (bind _itneracttipwidget (`self.ItneractTipWidget`)
        (:`then`
          (`Widget.SetVisibility` _itneracttipwidget "Collapsed"))
        (:`else`)))))

(fn `LoopCheckTarget`
  (bind (_success _actor) (`self.GetCloestActor`))
  ;[1 1 1] 先清空
  (`KismetArrayLibrary.Array_Clear` (`self.InteractiveActorList`))
  ;[1 1 1] 重叠检测
  (bind _outactors (`KismetSystemLibrary.SphereOverlapActors` (`Actor.K2_GetActorLocation` (`self.OwnerCharacter`)) (`self.InteractiveRadius`) (`|MakeArray` "ObjectTypeQuery3" "ObjectTypeQuery8" "ObjectTypeQuery1" "ObjectTypeQuery2" :!type "EObjectTypeQuery Enum") null (`|MakeArray` (`self.OwnerCharacter`) :!type "Actor Object Reference")))
  (for _array_element _outactors
    ;[1 1 1] 是否能够互动
    (`self.HasInterface` _array_element
      (:`真`
        (`self.CanInteract` _array_element
          (:`真`
            ;[1 1 1] 加入到互动物体列表
            (`KismetArrayLibrary.Array_AddUnique` (`self.InteractiveActorList`) _array_element))))))
  ;[1 1 1] 计算距离最近的可互动物体 添加互动提示
  (if _success
    (bind _output_get (set `self.CurrentTarget` _actor))
    (`self.IsMannulInteract` _output_get ; 需要手动互动？
      (:`真`
        (`self.ShowTip`))
      (:`false`
        (`self.HideTip`)))
    (else
      ;;[1 0.5252 0] 清空并隐藏
      (set `self.CurrentTarget` null)
      (`self.HideTip`))))

(fn `LoopLongPressInteract`
  (bind _currenttarget (`self.CurrentTarget`)
    (:`then`
      (bind _interactioninfo (message `/Game/BA_Rougelike/Blueprints/BPI/BPI_InteractiveObject.Get_InteractionInfo` _currenttarget))
      ;[1 1 1] 交互时间自增
      (bind _output_get (set `self.CurInteractTime` (+ (`self.CurInteractTime`) 0.1)))
      (bind ((`MaxInteractTime_16_B471BC834708071E62BA9CB17D447042` _maxinteracttime)) (break `/Game/BA_Rougelike/GameData/Structs/S_InteractionInfo` _interactioninfo))
      (`self.UpdateInteractProgess` (/ _output_get _maxinteracttime)) ; 更新交互进度
      (if (>= _output_get _maxinteracttime)
        ;[1 1 1] 激活交互
        (message `/Game/BA_Rougelike/Blueprints/BPI/BPI_InteractiveObject.ActiveInteraction` (`self.CurrentTarget`) (`self.OwnerCharacter`))
        (`self.EndLongPressInteract`)))
    (:`else`
      (`self.EndLongPressInteract`))))

(fn `SetIconScale`
  (params (Scale :type "Float (double-precision)"))
  (bind _returnvalue (* 30.0 (`local.Scale`)))
  (bind _itneracttipwidget (`self.ItneractTipWidget`)
    (:`then`
      (bind _iconsizebox (`/Game/BA_Rougelike/Blueprints/UMG/WBP_InteractTip.IconSizeBox` _itneracttipwidget))
      (set `SizeBox.WidthOverride` _returnvalue _iconsizebox)
      (set `SizeBox.HeightOverride` _returnvalue _iconsizebox))
    (:`else`)))

(fn `ShowTip`
  (`self.OwnerIsPlayer` ; 仅玩家
    (:`then`
      (bind _currenttarget (`self.CurrentTarget`)
        (:`then`
          (bind _itneracttipwidget (`self.ItneractTipWidget`)
            (:`then`
              (`Widget.SetVisibility` _itneracttipwidget "SelfHitTestInvisible")
              ;[1 1 1] 更新UI提示位置
              (`UserWidget.SetPositionInViewport` (`self.ItneractTipWidget`) (`GameplayStatics.ProjectWorldToScreen` (`GameplayStatics.GetPlayerController` 0) (`Actor.K2_GetActorLocation` _currenttarget)) true)
              ;[1 1 1] 更新提示文本
              (bind _interactioninfo (message `/Game/BA_Rougelike/Blueprints/BPI/BPI_InteractiveObject.Get_InteractionInfo` (`self.CurrentTarget`)))
              (`TextBlock.SetText` (`/Game/BA_Rougelike/Blueprints/UMG/WBP_InteractTip.InteractText` (`self.ItneractTipWidget`)) (`.InteractText_14_09C87E534BD16D04C8DDF3865F5D5FE5` (break `/Game/BA_Rougelike/GameData/Structs/S_InteractionInfo` _interactioninfo))))
            (:`else`)))
        (:`else`)))))

(fn `StartLongPressInteract`
  (`self.EndLongPressInteract`)
  (bind _returnvalue (`KismetSystemLibrary.K2_SetTimer` null "LoopLongPressInteract" 0.1 true true))
  (set `self.LongPressInteractFun` _returnvalue)
  (`self.SetIconScale` 1.2))

(fn `UpdateInteractProgess`
  (params (Precent :type "Float (single-precision)"))
  (bind _itneracttipwidget (`self.ItneractTipWidget`)
    (:`then`
      (set `ProgressBar.Percent` (`local.Precent`) (`/Game/BA_Rougelike/Blueprints/UMG/WBP_InteractTip.InteractProgess` _itneracttipwidget)))
    (:`else`)))