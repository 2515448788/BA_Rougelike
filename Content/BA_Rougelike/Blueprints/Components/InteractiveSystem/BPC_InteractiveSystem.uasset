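; Character component that tracks nearby interactable actors for the player and marks the closest with a floating tip.
; After the player-controlled owner finishes BeginPlay, it adds an overlap sphere and spawns one BP_InteractTip.
; Sphere overlaps maintain a list of BPI_InteractiveObject implementers and re-pick the nearest only when that list updates.
; The tip is reused, attached to the target or detached and parked below the world origin.
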(event `self.ReceiveBeginPlay`
  (`self.GetOwnerCharacter`)
  (`self.IsPlayer` ; 是否为玩家
    (:`真`
      (bind _ownercharacter (`self.OwnerCharacter`)
        (:`then`
          (add `/Game/BA_Rougelike/Blueprints/Characters/BP_MyCharacter_Base.OnBeginPlayComplete` _ownercharacter (delegate `BeginPlayComplete`)))
        (:`else`)))))

(event `BeginPlayComplete`
  (`self.AddSphereOverlap`)
  (`self.SpawnTip`))

(fn `AddSphereOverlap`
  (bind _returnvalue (`|AddComponentByClass` :`self` (`self.OwnerCharacter`) :`Class` "/Script/Engine.SphereComponent"))
  (set `self.InteractiveSphere` _returnvalue)
  (`SphereComponent.SetSphereRadius` (`self.InteractiveSphere`) (`self.InteractiveRadius`) true)
  (`PrimitiveComponent.SetCollisionProfileName` (`self.InteractiveSphere`) "ForPawnOverlap" true)
  (add `PrimitiveComponent.OnComponentBeginOverlap` (`self.InteractiveSphere`) (`|CreateDelegate` :!event `OnBeginOverlap`))
  (add `PrimitiveComponent.OnComponentEndOverlap` (`self.InteractiveSphere`) (`|CreateDelegate` :!event `OnEndOverlap`)))

(fn `GetCloestInteractiveActor`
  (returns (Success :type Boolean) (Actor :type "Actor Object Reference"))
  (locals (Distance :type "Float (double-precision)" :default 0.0) (IsFind :type Boolean) (CloestActor :type "Actor Object Reference"))
  (bind _interactiveactorlist (`self.InteractiveActorList`))
  (set `local.Distance` 999999999.0)
  (set `local.IsFind` false)
  (if (`KismetArrayLibrary.Array_IsNotEmpty` _interactiveactorlist)
    (for _array_element _interactiveactorlist
      (bind _returnvalue (`Actor.GetDistanceTo` _array_element (`self.OwnerCharacter`)))
      (if (< _returnvalue (`local.Distance`))
        (set `local.Distance` _returnvalue)
        (set `local.CloestActor` _array_element)
        (set `local.IsFind` true)))
    ;[1 1 1] 返回
    (return (`local.IsFind`) (`local.CloestActor`))
    (else
      ;[1 1 1] 失败 返回
      (return false null))))

(fn `GetOwnerCharacter`
  (bind _asbp_my_character_base (cast `/Game/BA_Rougelike/Blueprints/Characters/BP_MyCharacter_Base` (`self.GetOwner`)))
  (set `self.OwnerCharacter` _asbp_my_character_base))

(fn `HideTip`
  (`Actor.K2_DetachFromActor` (`self.InteractTip`) "KeepRelative" "KeepRelative" "KeepRelative")
  (`Actor.K2_SetActorLocation` (`self.InteractTip`) (0.0 0.0 -1000.0) false false)
  (`SceneComponent.K2_SetRelativeLocation` (`/Game/BA_Rougelike/Blueprints/Components/InteractiveSystem/BP_InteractTip.TipWidget` (`self.InteractTip`)) (0.0 0.0 0.0) false false))

(fn `OnBeginOverlap`
  (params (OverlappedComponent :type "PrimitiveComponent Object Reference") (OtherActor :type "Actor Object Reference") (OtherComp :type "PrimitiveComponent Object Reference") (OtherBodyIndex :type Integer) (bFromSweep :type Boolean) (SweepResult :type "HitResult Structure (by ref)"))
  (`self.ActorHasInterface` OtherActor ; 是否实现了互动接口
    (:`真`
      (`KismetArrayLibrary.Array_AddUnique` (`self.InteractiveActorList`) OtherActor)
      (`self.UpdateInteractTarget`)
      (return))))

(fn `OnEndOverlap`
  (params (OverlappedComponent :type "PrimitiveComponent Object Reference") (OtherActor :type "Actor Object Reference") (OtherComp :type "PrimitiveComponent Object Reference") (OtherBodyIndex :type Integer))
  (`self.ActorHasInterface` OtherActor ; 是否实现了互动接口
    (:`真`
      (bind _returnvalue (`KismetArrayLibrary.Array_RemoveItem` (`self.InteractiveActorList`) OtherActor))
      (if _returnvalue
        (`self.UpdateInteractTarget`)))))

(fn `ShowTip`
  (params (ParentActor :type "Actor Object Reference"))
  (bind _returnvalue (`Actor.K2_AttachToActor` (`self.InteractTip`) ParentActor "None" "SnapToTarget" "SnapToTarget" "SnapToTarget" true))
  (if _returnvalue
    (`SceneComponent.K2_SetRelativeLocation` (`/Game/BA_Rougelike/Blueprints/Components/InteractiveSystem/BP_InteractTip.TipWidget` (`self.InteractTip`)) (0.0 0.0 20.0) false false)))

(fn `SpawnTip`
  (bind _returnvalue (`|SpawnActorFromClass` "/Game/BA_Rougelike/Blueprints/Components/InteractiveSystem/BP_InteractTip.BP_InteractTip_C" (`KismetMathLibrary.MakeTransform` (0.0 0.0 -1000.0)) "AlwaysSpawn" "MultiplyWithRoot" null null))
  (set `self.InteractTip` _returnvalue))

(fn `UpdateInteractTarget`
  (bind (_success _actor) (`self.GetCloestInteractiveActor`))
  (if _success
    (`self.ShowTip` _actor)
    (else
      (`self.HideTip`))))