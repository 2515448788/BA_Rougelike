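; Actor component that shows floating damage numbers whenever its owning Character takes damage.
; On BeginPlay it caches the owner as a Character and binds to OnTakeAnyDamage.
; Each hit pulls a BP_FloatingDamage actor from the pool subsystem at the owner's location plus a random per-axis offset, then plays its normal animation with the damage value.
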(event `self.ReceiveBeginPlay`
  (bind `_as角色` (cast `Character` (`self.GetOwner`)))
  (bind _output_get (set `self.OwnerCharacter` `_as角色`))
  (add `Actor.OnTakeAnyDamage` _output_get (`|CreateDelegate` :!event `OnTakeAnyDamage`)))

(fn `OnTakeAnyDamage`
  (params (DamagedActor :type "Actor Object Reference") (Damage :type "Float (single-precision)") (DamageType :type "DamageType Object Reference") (InstigatedBy :type "Controller Object Reference") (DamageCauser :type "Actor Object Reference"))
  (bind _offsetmin (`self.OffsetMin`))
  (bind _offsetmax (`self.OffsetMax`))
  (bind _ownercharacter (`self.OwnerCharacter`)
    (:`then`
      (bind _spawnedactor (`PoolSubsystem.SpawnFromPool` :`self` (subsystem `PoolSubsystem`) :`PoolClass` "/Game/BA_Rougelike/Blueprints/Components/FloatingDamage/BP_FloatingDamage.BP_FloatingDamage_C" :`Location` (+ (`Actor.K2_GetActorLocation` _ownercharacter) (`KismetMathLibrary.MakeVector` (`KismetMathLibrary.RandomFloatInRange` _offsetmin _offsetmax) (`KismetMathLibrary.RandomFloatInRange` _offsetmin _offsetmax) (`KismetMathLibrary.RandomFloatInRange` _offsetmin _offsetmax)))))
      (`/Engine/EditorBlueprintResources/StandardMacros.IsValid` _spawnedactor
        (:`Is Valid`
          (`/Game/BA_Rougelike/Blueprints/Components/FloatingDamage/BP_FloatingDamage.PlayNormalAnimation` _spawnedactor Damage))))
    (:`else`)))