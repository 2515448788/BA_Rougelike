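; BP_FloatingDamage is a pooled actor that displays animated floating damage numbers through a widget component.
; It caches its WBP_FloatingDamage widget on BeginPlay and forwards normal or critical damage values to the matching widget animation.
; On spawn from the pool it enables tick and binds to animation completion, which returns it to the pool subsystem.
; On return it stops all animations and disables tick.
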(event `self.ReceiveBeginPlay`
  (bind _damagewidget (`self.DamageWidget`)
    (:`then`
      (bind _aswbp_floating_damage (cast `/Game/BA_Rougelike/Blueprints/UMG/WBP_FloatingDamage` (`WidgetComponent.GetUserWidgetObject` _damagewidget)))
      (set `self.DamageWidgetObject` _aswbp_floating_damage))
    (:`else`)))

(event `PlayNormalAnimation`
  (params (Damage :type "Float (double-precision)"))
  (bind _damagewidgetobject (`self.DamageWidgetObject`)
    (:`then`
      (message `/Game/BA_Rougelike/GameData/BPI/BPI_FloatingDamage.PlayNormalAnimation` _damagewidgetobject Damage))
    (:`else`)))

(event `PlayCriticallAnimation`
  (params (Damage :type "Float (double-precision)"))
  (bind _damagewidgetobject (`self.DamageWidgetObject`)
    (:`then`
      (message `/Game/BA_Rougelike/GameData/BPI/BPI_FloatingDamage.PlayCriticallAnimation` _damagewidgetobject Damage))
    (:`else`)))

(event `PoolableInterface.OnSpawnFromPool`
  (bind _damagewidgetobject (`self.DamageWidgetObject`)
    (:`then`
      (`self.SetActorTickEnabled` true)
      (add `/Game/BA_Rougelike/Blueprints/UMG/WBP_FloatingDamage.AnimationPlayComplete` _damagewidgetobject (delegate `OnPlayComplete`)))
    (:`else`)))

(event `OnPlayComplete`
  ;[1 1 1] 回到对象池
  (`PoolSubsystem.ReturnToPool` (subsystem `PoolSubsystem`) self))

(event `PoolableInterface.OnReturnToPool`
  (bind _damagewidgetobject (`self.DamageWidgetObject`)
    (:`then`
      (`UserWidget.StopAllAnimations` _damagewidgetobject)
      (`self.SetActorTickEnabled` false))
    (:`else`)))

(fn `UserConstructionScript`)