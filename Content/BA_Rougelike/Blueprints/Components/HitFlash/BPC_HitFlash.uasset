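; Character component that flashes the owner's mesh with a colored glow whenever it takes damage.
; On BeginPlay it creates a dynamic hit-flash material instance, sets it as the character mesh's overlay material and binds to OnTakeAnyDamage.
; Flash sets color, strength and alpha, then clears them after a retriggerable delay, so repeated hits extend the flash.
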(event `self.ReceiveBeginPlay`
  ;[1 1 1] 初始化
  (bind `_as角色` (cast `Character` (`self.GetOwner`)))
  (set `self.OwnerCharacter` `_as角色`)
  (`self.CreateOverlayMaterial`)
  (add `Actor.OnTakeAnyDamage` (`self.OwnerCharacter`) (`|CreateDelegate` :!event `OnTakeAnyDamage`)))

(event `Flash`
  (params (Color :type "LinearColor Structure") (Strength :type "Float (single-precision)") (Alpha :type "Float (single-precision)") (Time :type "Float (single-precision)"))
  ;[1 1 1] 闪光一次
  (bind _flashmaterial (`self.FlashMaterial`)
    (:`then`
      (`MaterialInstanceDynamic.SetVectorParameterValue` _flashmaterial "EmissiveColor" Color)
      (`MaterialInstanceDynamic.SetScalarParameterValue` (`self.FlashMaterial`) "EmissiveMultiplier" Strength)
      (`MaterialInstanceDynamic.SetScalarParameterValue` (`self.FlashMaterial`) "Alpha" Alpha)
      (`KismetSystemLibrary.RetriggerableDelay` Time)
      (`MaterialInstanceDynamic.SetVectorParameterValue` :`self` (`self.FlashMaterial`) :`ParameterName` "EmissiveColor")
      (`MaterialInstanceDynamic.SetScalarParameterValue` (`self.FlashMaterial`) "EmissiveMultiplier" 0.0)
      (`MaterialInstanceDynamic.SetScalarParameterValue` (`self.FlashMaterial`) "Alpha" 0.0))
    (:`else`)))

(fn `CreateOverlayMaterial`
  (bind _ownercharacter (`self.OwnerCharacter`)
    (:`then`
      (bind _mesh (`Character.Mesh` _ownercharacter)
        (:`then`
          ;[1 1 1] 创建动态材质实例
          (bind _returnvalue (`KismetMaterialLibrary.CreateDynamicMaterialInstance` "/Game/BA_Rougelike/Materials/MI_HitFlashInst.MI_HitFlashInst"))
          (bind _output_get (set `self.FlashMaterial` _returnvalue))
          (`MeshComponent.SetOverlayMaterial` _mesh _output_get))
        (:`else`)))
    (:`else`)))

(fn `OnTakeAnyDamage`
  (params (DamagedActor :type "Actor Object Reference") (Damage :type "Float (single-precision)") (DamageType :type "DamageType Object Reference") (InstigatedBy :type "Controller Object Reference") (DamageCauser :type "Actor Object Reference"))
  (`self.Flash` (`self.FlashColor_TakeDmage`) (`self.FlashStrength_TakeDmage`) (`self.FlashAlpha_TakeDmage`) (`self.FlashTime_TakeDmage`)))