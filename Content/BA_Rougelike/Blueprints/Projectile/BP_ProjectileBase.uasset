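; Base pooled projectile that damages what it hits, spawns a Niagara impact effect and returns to the pool.
; Pool spawn and return events share one reset chain, branched by IsReturnToPool, that toggles owner, ignore-owner movement, trail FX, movement, collision and velocity.
; On spawn it caches damage and instigator controller from its owner.
; A lifetime timer returns unspent projectiles to the pool and is cleared on return.
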(event `PoolableInterface.OnSpawnFromPool`
  ;[1 1 1] 对象池处理
  (set `self.IsReturnToPool` false)
  (`self.RsetOwner` :!label _label) ; 重置拥有者
  (`self.ResetIgnoreMoving`) ; 重置-移动时忽略Actor
  (`self.ResetFX`) ; 重置-特效
  (`self.ResetProjectileMovement`) ; 重置-移动组件
  (`self.ResetCollision`) ; 重置-碰撞
  (`self.ResetDestorySelf`) ; 重置-自毁倒计时
  (`self.ResetVelocity`) ; 重置-速度
  (`self.ResetDamage`) ; 重置-本次伤害
)

(event `PoolableInterface.OnReturnToPool`
  ;[1 1 1] 对象池处理
  (set `self.IsReturnToPool` true)
  (goto _label))

(event `self.Sphere.OnComponentHit`
  (params (HitComponent :type "PrimitiveComponent Object Reference") (OtherActor :type "Actor Object Reference") (OtherComp :type "PrimitiveComponent Object Reference") (NormalImpulse :type "Vector Structure") (Hit :type "HitResult Structure (by ref)"))
  ;[1 1 1] 命中时
  (`self.ApplyDamage` OtherActor) ; 伤害
  (`self.HitVFX` Hit) ; 命中特效
  (`self.ReturnToPool`) ; 回到对象池
)

(fn `ApplyDamage`
  (params (DamagedActor :type "Actor Object Reference"))
  (`GameplayStatics.ApplyDamage` (`local.DamagedActor`) (`self.LocalDamage`) (`self.CurlInstigatorCaontroller`) self "/Game/BA_Rougelike/Blueprints/DamageType/BP_DamageBase.BP_DamageBase_C"))

(fn `HitVFX`
  (params (Hit :type "HitResult Structure"))
  (bind (_bblockinghit _binitialoverlap _time _distance _location _impactpoint _normal _impactnormal) (`GameplayStatics.BreakHitResult` Hit))
  (`NiagaraFunctionLibrary.SpawnSystemAtLocation` (`self.VFXHit`) _impactpoint (`KismetMathLibrary.MakeRotFromX` _impactnormal) (* (`self.VFXHitScale`) (`KismetMathLibrary.MakeVector` 1.0 1.0 1.0)) true true "AutoRelease"))

(fn `ResetCollision`
  (`PrimitiveComponent.SetCollisionProfileName` (`self.Sphere`) (select `bool` (`self.IsReturnToPool`) :`false` "Projectile" :`true` "NoCollision" :!type "Name") true))

(fn `ResetDamage`
  (bind _returnvalue (`self.GetOwner`))
  (`/Engine/EditorBlueprintResources/StandardMacros.IsValid` _returnvalue
    (:`Is Valid`
      (set `self.LocalDamage` (select `bool` (`self.IsReturnToPool`) :`false` (`/Game/BA_Rougelike/Blueprints/BFL/BFL_Common.GetActorDamage` _returnvalue))))
    (:`Is Not Valid`
      (set `self.LocalDamage` 0.0))))

(fn `ResetDestorySelf`
  (if (`self.IsReturnToPool`)
    ;[1 1 1] 清除自毁倒计时
    (`KismetSystemLibrary.K2_ClearAndInvalidateTimerHandle` (`self.ReturnToPoolHandle`))
    (else
      ;[1 1 1] 自毁倒计时
      (bind _returnvalue (`KismetSystemLibrary.K2_SetTimer` null "ReturnToPool" (`self.MaxLifeTime`)))
      (set `self.ReturnToPoolHandle` _returnvalue))))

(fn `ResetFX`
  (bind _niagara (`self.Niagara`))
  (if (`self.IsReturnToPool`)
    (`ActorComponent.Deactivate` _niagara)
    (else
      (`ActorComponent.Activate` _niagara true))))

(fn `ResetIgnoreMoving`
  (`PrimitiveComponent.IgnoreActorWhenMoving` (`self.Sphere`) (`self.GetOwner`) (select `bool` (`self.IsReturnToPool`) :`false` true)))

(fn `ResetProjectileMovement`
  (`MovementComponent.SetUpdatedComponent` (`self.ProjectileMovement`) (select `bool` (`self.IsReturnToPool`) :`false` (`self.RootComponent`))))

(fn `ResetVelocity`
  (set `MovementComponent.Velocity` (select `bool` (`self.IsReturnToPool`) :`false` (* (`KismetMathLibrary.GetForwardVector` (`self.K2_GetActorRotation`)) (`ProjectileMovementComponent.InitialSpeed` (`self.ProjectileMovement`)))) (`self.ProjectileMovement`)))

(fn `ReturnToPool`
  ;[1 1 1] 回到对象池
  (`PoolSubsystem.ReturnToPool` (subsystem `PoolSubsystem`) self))

(fn `RsetOwner`
  (bind _output_get (set `self.CurOwner` (select `bool` (`self.IsReturnToPool`) :`false` (`self.GetOwner`))))
  (`/Engine/EditorBlueprintResources/StandardMacros.IsValid` _output_get
    (:`Is Valid`
      (set `self.CurlInstigatorCaontroller` (`self.GetInstigatorController` _output_get)))))

(fn `UserConstructionScript`)