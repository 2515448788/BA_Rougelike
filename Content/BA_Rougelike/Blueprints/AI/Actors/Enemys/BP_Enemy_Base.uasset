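; Base enemy character for the roguelike, providing melee-style attacks, health and death, plus getters and setters for combat stats and group.
; NormalAttack turns toward the player on a timeline, plays a montage, then waits out a cooldown.
; Damage is processed through the DamageType; death stops AI logic, disables collision, hides the mesh and returns the actor to a pool.
; Pool spawn and return hooks restore that state and update group subsystem registration.
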(event `/Game/BA_Rougelike/Blueprints/BPI/BPI_Enemy.NormalAttack`
  ;[1 1 1] 普通攻击
  (if (not (`self.IsAttackCooldown`))
    (set `self.IsAttackCooldown` true) ; 设置冷却
    (bind (_direction _alpha) (`Timeline|TL_RotateToPlayer` :!via `PlayFromStart`)
      (:`Update`
        (`self.RotateToPlayer` _alpha))
      (:`Finished`
        (bind _attackmontage (`self.AttackMontage`) ; 蒙太奇是否有效
          (:`then`
            (`self.PlayAnimMontage` _attackmontage))
          (:`else`
            _))
        ;;[1 1 1] 攻击冷却逻辑
        (`KismetSystemLibrary.Delay` (`self.AttackInterval`))
        (set `self.IsAttackCooldown` false)))))

(event `/Game/BA_Rougelike/Blueprints/BPI/BPI_Enemy.Set_IsAttackState`
  (params (IsAttackState :type Boolean))
  ;[1 1 1] 攻击状态控制
  (set `self.IsInAttackState` IsAttackState))

(event `self.ReceiveAnyDamage`
  (params (Damage :type "Float (single-precision)") (DamageType :type "DamageType Object Reference") (InstigatedBy :type "Controller Object Reference") (DamageCauser :type "Actor Object Reference"))
  (bind _damageout (message `/Game/BA_Rougelike/Blueprints/BPI/BPI_DamageType.ProcessDamage` DamageType Damage self InstigatedBy))
  (`self.ChangeCurHealthValue` _damageout) ; 修改生命值
  (`self.IsDeath`
    (:`true`
      ;[1 1 1] 死亡时延迟一秒回对象池
      (`self.ResetAI`)
      (`self.ResetCollision`)
      (`self.ResetMeshVisibility`)
      (`KismetSystemLibrary.Delay` 0.5)
      (`self.ReturnToPool`))))

(event `PoolableInterface.OnSpawnFromPool`
  (`self.InitAI`)
  (`self.InitMeshVisibility`)
  (`self.InitCollision`)
  (`self.InitGroupMap`))

(event `PoolableInterface.OnReturnToPool`
  (`self.ResetGroupMap`))

(event `/Game/BA_Rougelike/Blueprints/BPI/BPI_Enemy.Set_Health`
  (params (CurHealth :type "Float (double-precision)") (MaxHealth :type "Float (double-precision)"))
  ;[1 1 1] 重载生命值
  (set `self.CurHealth` CurHealth)
  (set `self.MaxHealth` MaxHealth))

(event `/Game/BA_Rougelike/Blueprints/BPI/BPI_Enemy.Set_Damage`
  (params (NewDamage :type "Float (double-precision)"))
  ;[1 1 1] 重载伤害
  (set `self.AttackDamage` NewDamage))

(event `/Game/BA_Rougelike/Blueprints/BPI/BPI_CharacterCommon.Set_Group`
  (params (NewGroup :type "/Game/BA_Rougelike/GameData/Enums/E_ActorGroup Enum" :default "NewEnumerator0"))
  ;[1 1 1] 重载组
  (set `self.Group` NewGroup))

(event `/Game/BA_Rougelike/Blueprints/BPI/BPI_CharacterCommon.Set_MoveIgnoreActor`
  (params (Actor :type "Actor Object Reference") (ShouldIgnore :type Boolean))
  ;[1 1 1] 设置移动时忽略Actor
  (`PrimitiveComponent.IgnoreActorWhenMoving` (`self.CapsuleComponent`) Actor ShouldIgnore)
  (`PrimitiveComponent.IgnoreActorWhenMoving` (`self.Mesh`) Actor ShouldIgnore))

(fn `ChangeCurHealthValue`
  (params (Damage :type "Float (double-precision)"))
  (locals (LocalOldCurHealth :type "Float (double-precision)" :default 0.0))
  (bind _curhealth (`self.CurHealth`))
  (set `local.LocalOldCurHealth` _curhealth)
  (bind _output_get (set `self.CurHealth` (`KismetMathLibrary.FClamp` (- _curhealth Damage) 0.0 (`self.MaxHealth`))))
  (`self.CurHealthChanged` (`local.LocalOldCurHealth`) _output_get))

(fn `Get_ArmorType`
  (returns (ArmorType :type "/Game/BA_Rougelike/GameData/Enums/E_ArmorType Enum"))
  (return (`self.ArmorType`)))

(fn `Get_AttackInterval`
  (returns (AttackInterval :type "Float (double-precision)"))
  (return (`self.AttackInterval`)))

(fn `Get_AttackMontage`
  (returns (Montage :type "AnimMontage Object Reference"))
  (return (`self.AttackMontage`)))

(fn `Get_AttackRange`
  (returns (Range :type "Float (double-precision)"))
  (return (`self.AttackRange`)))

(fn `Get_AttackType`
  (returns (AttackType :type "/Game/BA_Rougelike/GameData/Enums/E_AttackType Enum"))
  (return (`self.AttackType`)))

(fn `Get_Damage`
  (returns (Damage :type "Float (double-precision)"))
  (return (`self.AttackDamage`)))

(fn `Get_Group`
  (returns (Group :type "/Game/BA_Rougelike/GameData/Enums/E_ActorGroup Enum"))
  (return (`self.Group`)))

(fn `Get_Health`
  (returns (CurHealth :type "Float (double-precision)") (MaxHealth :type "Float (double-precision)"))
  (return (`self.CurHealth`) (`self.MaxHealth`)))

(fn `Get_IsAttackState`
  (returns (IsInAttackState :type Boolean))
  (return (`self.IsInAttackState`)))

(fn `Get_MoveSpeed`
  (returns (MoveSpeed :type "Float (double-precision)"))
  (return (`self.MoveSpeed`)))

(fn `InitAI`
  (bind _returnvalue (`AIBlueprintHelperLibrary.GetAIController` self))
  (`/Engine/EditorBlueprintResources/StandardMacros.IsValid` _returnvalue
    (:`Is Valid`
      (`BrainComponent.RestartLogic` (`AIController.BrainComponent` _returnvalue)))))

(fn `InitCollision`
  (`PrimitiveComponent.SetCollisionProfileName` (`self.CapsuleComponent`) "Pawn" true)
  (`PrimitiveComponent.SetCollisionProfileName` (`self.Mesh`) "CharacterMesh" true))

(fn `InitGroupMap`
  (`/Game/BA_Rougelike/Blueprints/SubSystem/BP_GroupSubsystem.RegisterToMap` (subsystem `/Game/BA_Rougelike/Blueprints/SubSystem/BP_GroupSubsystem`) self))

(fn `InitHealth`
  (set `self.CurHealth` (`self.MaxHealth`)))

(fn `InitMeshVisibility`
  (`SceneComponent.SetVisibility` (`self.Mesh`) true false))

(fn `InitMoveSpeed`
  ;[1 1 1] 初始化移动速度
  (set `CharacterMovementComponent.MaxWalkSpeed` (`self.MoveSpeed`) (`self.CharacterMovement`)))

(fn `ResetAI`
  (bind _returnvalue (`AIBlueprintHelperLibrary.GetAIController` self))
  (`/Engine/EditorBlueprintResources/StandardMacros.IsValid` _returnvalue
    (:`Is Valid`
      (`BrainComponent.StopLogic` (`AIController.BrainComponent` _returnvalue) "Dead"))))

(fn `ResetCollision`
  (`PrimitiveComponent.SetCollisionProfileName` (`self.CapsuleComponent`) "NoCollision" true)
  (`PrimitiveComponent.SetCollisionProfileName` (`self.Mesh`) "NoCollision" true))

(fn `ResetGroupMap`
  (`/Game/BA_Rougelike/Blueprints/SubSystem/BP_GroupSubsystem.RemoveFromMap` (subsystem `/Game/BA_Rougelike/Blueprints/SubSystem/BP_GroupSubsystem`) self))

(fn `ResetMeshVisibility`
  (`SceneComponent.SetVisibility` (`self.Mesh`) false false))

(fn `ReturnToPool`
  ;[1 1 1] 返回对象池
  (`PoolSubsystem.ReturnToPool` (subsystem `PoolSubsystem`) self))

(fn `RotateToPlayer`
  (params (Alpha :type "Float (single-precision)"))
  (`self.K2_SetActorRotation` (`KismetMathLibrary.RLerp` (`self.K2_GetActorRotation`) (`KismetMathLibrary.FindLookAtRotation` (`self.K2_GetActorLocation`) (`self.K2_GetActorLocation` (`GameplayStatics.GetPlayerPawn` 0))) Alpha true)))

(fn `UserConstructionScript`
  (`self.InitMoveSpeed`))