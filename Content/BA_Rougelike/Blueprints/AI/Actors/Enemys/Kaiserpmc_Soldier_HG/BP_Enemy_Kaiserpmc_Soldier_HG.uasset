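; Enemy Blueprint for a Kaiser PMC soldier (HG variant) that fires projectiles at the player.
; On the normal attack anim notify, it requests a BP_ProjectileBase from the pool subsystem at the muzzle socket, rotated toward player pawn 0.
; Each shot also draws a one-second debug arrow from muzzle to player.
; The construction script only calls the parent.
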(event `/Game/BA_Rougelike/Blueprints/BPI/BPI_AI.NormalAttack_AnimNotify`
  (bind _returnvalue (`SceneComponent.GetSocketLocation` (`self.Mesh`) "Socket_Muzzle"))
  (bind _returnvalue_2 (`self.K2_GetActorLocation` (`GameplayStatics.GetPlayerPawn` 0)))
  (`KismetSystemLibrary.DrawDebugArrow` _returnvalue _returnvalue_2 10.0 (struct :`R` 1.0 :`B` 0.048514 :`A` 1.0) 1.0 1.0)
  (`PoolSubsystem.SpawnFromPool` (subsystem `PoolSubsystem`) "/Game/BA_Rougelike/Blueprints/Projectile/BP_ProjectileBase.BP_ProjectileBase_C" _returnvalue (`KismetMathLibrary.FindLookAtRotation` _returnvalue _returnvalue_2) self))

(fn `UserConstructionScript`
  (`parent.UserConstructionScript`))