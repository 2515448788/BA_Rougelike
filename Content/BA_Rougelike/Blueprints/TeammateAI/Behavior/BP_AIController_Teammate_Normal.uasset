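; AI controller for normal teammates that holds a current combat target and turns the pawn to face it.
; Interface events set or clear the target along with focus, and a getter exposes it.
; Each tick, while the target has health above zero, it smoothly interpolates control-rotation yaw toward it and messages the pawn to switch rotate mode.
; Without a valid living target, it sets the pawn to the other rotate mode.
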(event `self.ReceiveTick`
  (params (DeltaSeconds :type "Float (single-precision)"))
  (set `self.Delta Seconds` DeltaSeconds)
  (bind _targetactor (`self.TargetActor`)
    (:`then`
      (`self.LookAtTargetActor` _targetactor))
    (:`else`
      (message `/Game/BA_Rougelike/Blueprints/BPI/BPI_PlayerCharacter.Set_RotateMode` (`self.K2_GetPawn`) "NewEnumerator0"))))

(event `/Game/BA_Rougelike/Blueprints/BPI/BPI_PlayerController.Clear_CurrentTarget`
  (set `self.TargetActor` null)
  (`self.K2_ClearFocus`))

(event `/Game/BA_Rougelike/Blueprints/BPI/BPI_PlayerController.Set_CurrentTarget`
  (params (TargetActor :type "Actor Object Reference"))
  (bind _output_get (set `self.TargetActor` TargetActor))
  (`self.K2_SetFocus` _output_get)
  (`self.K2_SetFocalPoint` (`self.K2_GetActorLocation` _output_get)))

(fn `Get_BaseCanvas`
  (returns (UserBaseCanvas :type "/Game/BA_Rougelike/Blueprints/UMG/WBP_UserBaseCanvas Object Reference"))
  (return null))

(fn `Get_CurrentTarget`
  (returns (CurTarget :type "Actor Object Reference"))
  (return (`self.TargetActor`)))

(fn `LookAtTargetActor`
  (params (TargetActor :type "Actor Object Reference"))
  (bind (_returnvalue_roll _returnvalue_pitch) (`KismetMathLibrary.BreakRotator` (`self.GetControlRotation`)))
  (bind (_returnvalue_roll_2 _returnvalue_pitch_2 _returnvalue_yaw) (`KismetMathLibrary.BreakRotator` (`KismetMathLibrary.RInterpTo` (`self.K2_GetActorRotation` (`self.K2_GetPawn`)) (`KismetMathLibrary.FindLookAtRotation` (`self.K2_GetActorLocation` (`self.K2_GetPawn`)) (`self.K2_GetActorLocation` TargetActor)) (`self.Delta Seconds`) 8.0)))
  (`/Engine/EditorBlueprintResources/StandardMacros.IsValid` TargetActor
    (:`Is Valid`
      (`self.IsTargetAlive` (`local.TargetActor`)
        (:`真`
          (`self.SetControlRotation` (`KismetMathLibrary.MakeRotator` _returnvalue_roll _returnvalue_pitch _returnvalue_yaw))
          (message `/Game/BA_Rougelike/Blueprints/BPI/BPI_PlayerCharacter.Set_RotateMode` (`self.K2_GetPawn`) "NewEnumerator1"))
        (:`false`
          (message `/Game/BA_Rougelike/Blueprints/BPI/BPI_PlayerCharacter.Set_RotateMode` (`self.K2_GetPawn`) "NewEnumerator0" :!label _label))))
    (:`Is Not Valid`
      (goto _label))))

(fn `UserConstructionScript`)