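; Base damage Blueprint that turns incoming damage into final damage, a matchup type and a critical flag.
; ProcessDamage looks up the instigator pawn's attack type against the damaged actor's armor type in a nested map, then scales damage by the matchup.
; ProcessCritical then rolls the instigator's float attributes for critical chance and multiplier.
; Failed instigator or matchup lookups return the damage unchanged as normal, non-critical.
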(fn `ProcessCritical`
  (params (DamageIn :type "Float (double-precision)") (Actor :type "Actor Object Reference"))
  (returns (DamageOut :type "Float (double-precision)") (IsCritical :type Boolean))
  (bind (_bsuccessfullyfoundattribute _returnvalue) (`AbilitySystemBlueprintLibrary.GetFloatAttribute` Actor (struct :`AttributeName` "CriticalChance" :`Attribute` "/Script/BA_Rougelike.MyAttributeSet_Character:CriticalChance" :`AttributeOwner` "/Script/CoreUObject.Class'/Script/BA_Rougelike.MyAttributeSet_Character'")))
  (bind (_bsuccessfullyfoundattribute_2 _returnvalue_2) (`AbilitySystemBlueprintLibrary.GetFloatAttribute` (`local.Actor`) (struct :`AttributeName` "CriticalMultiplier" :`Attribute` "/Script/BA_Rougelike.MyAttributeSet_Character:CriticalMultiplier" :`AttributeOwner` "/Script/CoreUObject.Class'/Script/BA_Rougelike.MyAttributeSet_Character'")))
  (if _bsuccessfullyfoundattribute
    (if (>= _returnvalue (`KismetMathLibrary.RandomFloatInRange` 0.0 1.0))
      (if _bsuccessfullyfoundattribute_2
        (return (* (`local.DamageIn`) _returnvalue_2) true)
        (else
          _))))
  ;[1 1 1] 原样返回
  (return (`local.DamageIn`) false))

(fn `ProcessDamage`
  (params (DamageIn :type "Float (double-precision)") (DamagedActor :type "Actor Object Reference") (InstigatorCaontroller :type "Controller Object Reference"))
  (returns (DamageOut :type "Float (double-precision)") (DamageType :type "/Game/BA_Rougelike/GameData/Enums/E_DamageType Enum") (IsCritical :type Boolean))
  (locals (LocalInstigarorPawn :type "Pawn Object Reference") (LocalDamageType :type "/Game/BA_Rougelike/GameData/Enums/E_DamageType Enum") (LocalFinalDamage :type "Float (double-precision)"))
  (`/Engine/EditorBlueprintResources/StandardMacros.IsValid` InstigatorCaontroller
    (:`Is Valid`
      (bind _output_get (set `local.LocalInstigarorPawn` (`Controller.K2_GetPawn` InstigatorCaontroller)))
      (`/Engine/EditorBlueprintResources/StandardMacros.IsValid` _output_get
        (:`Is Valid`
          ;[1 1 1] 计算最终伤害类型（普通 有利 弱点 半减）
          (bind _attacktype (message `/Game/BA_Rougelike/Blueprints/BPI/BPI_CharacterCommon.Get_AttackType` (`local.LocalInstigarorPawn`)))
          (bind (_value _returnvalue) (`BlueprintMapLibrary.Map_Find` (`self.DamageTypeMap`) _attacktype))
          (if _returnvalue
            (bind _armortype (message `/Game/BA_Rougelike/Blueprints/BPI/BPI_CharacterCommon.Get_ArmorType` (`local.DamagedActor`)))
            (bind (_value_2 _returnvalue_2) (`BlueprintMapLibrary.Map_Find` (`.ArmorDamageMap_4_B4DBEB6C431EF4AE82048FB53C1DD4C8` (break `/Game/BA_Rougelike/GameData/Structs/S_ArmorDamageType` _value)) _armortype))
            (if _returnvalue_2
              (bind _output_get_2 (set `local.LocalDamageType` _value_2))
              ;[1 1 1] 应用伤害倍率
              (bind _output_get_3 (set `local.LocalFinalDamage` (* (`local.DamageIn`) (select `/Game/BA_Rougelike/GameData/Enums/E_DamageType` _output_get_2 :`NewEnumerator4` 1.0 :`NewEnumerator0` 1.0 :`NewEnumerator1` 1.5 :`NewEnumerator2` 2.0 :`NewEnumerator3` 0.5))))
              ;[1 1 1] 处理暴击
              (bind (_damageout _iscritical) (`self.ProcessCritical` _output_get_3 (`local.LocalInstigarorPawn`)))
              (return _damageout (`local.LocalDamageType`) _iscritical)
              (else
                _))))
        (:`Is Not Valid`
          _)))
    (:`Is Not Valid`
      _))
  ;[1 1 1] 原样返回
  (return (`local.DamageIn`) "NewEnumerator0" false))