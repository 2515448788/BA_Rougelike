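; Group subsystem that tracks actors by group and returns the list of actors sharing a given actor's group.
; Registering and removing read the group enum from the actor's GetGroupMessage, edit that group's Actors collection and write the struct back into ActorGroupMap.
; Groups must already exist in the map: registration prints an error for a missing one, while removal skips it silently.
; An EnableDebug flag prints membership changes and counts.
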(fn `GetGroupMap`
  (returns (GroupMap :type "Map of /Game/BA_Rougelike/GameData/Enums/E_ActorGroup Enum to /Game/BA_Rougelike/GameData/Structs/S_GroupActorInfo Structure"))
  (return (`self.ActorGroupMap`)))

(fn `GetSameGroupActorList`
  (params (Actor :type "Actor Object Reference"))
  (returns (ActorList :type "Array of Actor Object Reference"))
  (bind _group (message `/Game/BA_Rougelike/Blueprints/BPI/BPI_CharacterCommon.Get_Group` Actor))
  (bind _value (`self.GetGroupInfo` _group)
    (:`true`
      (return (break `/Game/BA_Rougelike/GameData/Structs/S_GroupActorInfo` _value)))
    (:`false`
      (return))))

(fn `RegisterToMap`
  (params (Actor :type "Actor Object Reference"))
  (locals (LocalGroup :type "/Game/BA_Rougelike/GameData/Enums/E_ActorGroup Enum" :default "NewEnumerator0") (LocalGroupInfo :type "/Game/BA_Rougelike/GameData/Structs/S_GroupActorInfo Structure"))
  (bind _group (message `/Game/BA_Rougelike/Blueprints/BPI/BPI_CharacterCommon.Get_Group` Actor))
  (bind _output_get (set `local.LocalGroup` _group))
  (bind _value (`self.GetGroupInfo` _output_get)
    (:`true`
      ;[1 1 1] 更新替换组信息
      (bind _output_get_2 (set `local.LocalGroupInfo` _value))
      (`KismetArrayLibrary.Array_Add` (break `/Game/BA_Rougelike/GameData/Structs/S_GroupActorInfo` _output_get_2) (`local.Actor`))
      (`BlueprintMapLibrary.Map_Add` (`self.ActorGroupMap`) (`local.LocalGroup`) (`local.LocalGroupInfo`))
      ;[1 1 1] 调试
      (`self.IsEnableDebug`
        (:`真`
          (bind _value_2 (`self.GetGroupInfo` (`local.LocalGroup`))
            (:`true`
              (`KismetSystemLibrary.PrintString` (`KismetStringLibrary.Concat_StrStr` "GroupSubsystem: RegisterToMap   |" "| GroupName: " (`|GetEnumeratorNameAsString` (`local.LocalGroup`)) "| ActorName: " (`KismetSystemLibrary.GetDisplayName` (`local.Actor`)) "| Num: " (`KismetStringLibrary.Conv_IntToString` (`KismetArrayLibrary.Array_Length` (`.Actors_3_881F6EFA4F308E3FE4AA9FB5B124018A` (break `/Game/BA_Rougelike/GameData/Structs/S_GroupActorInfo` _value_2)))))))))))
    (:`false`
      ;[1 1 1] 日志
      (`KismetSystemLibrary.PrintString` (`KismetStringLibrary.Concat_StrStr` "角色组子系统： 未找到对应组的数据 检查变量初始化是否完整" (`|GetEnumeratorNameAsString` (`local.LocalGroup`)))))))

(fn `RemoveFromMap`
  (params (Actor :type "Actor Object Reference"))
  (locals (LocalGroup :type "/Game/BA_Rougelike/GameData/Enums/E_ActorGroup Enum" :default "NewEnumerator0") (LocalGroupInfo :type "/Game/BA_Rougelike/GameData/Structs/S_GroupActorInfo Structure"))
  (bind _group (message `/Game/BA_Rougelike/Blueprints/BPI/BPI_CharacterCommon.Get_Group` Actor))
  (bind _output_get (set `local.LocalGroup` _group))
  (bind _value (`self.GetGroupInfo` _output_get)
    (:`true`
      ;[1 1 1] 更新替换组信息
      (bind _output_get_2 (set `local.LocalGroupInfo` _value))
      (`KismetArrayLibrary.Array_RemoveItem` (break `/Game/BA_Rougelike/GameData/Structs/S_GroupActorInfo` _output_get_2) (`local.Actor`))
      (`BlueprintMapLibrary.Map_Add` (`self.ActorGroupMap`) (`local.LocalGroup`) (`local.LocalGroupInfo`))
      ;[1 1 1] 调试
      (`self.IsEnableDebug`
        (:`真`
          (bind _value_2 (`self.GetGroupInfo` (`local.LocalGroup`))
            (:`true`
              (`KismetSystemLibrary.PrintString` (`KismetStringLibrary.Concat_StrStr` "GroupSubsystem: RemoveFromMap   |" "| GroupName: " (`|GetEnumeratorNameAsString` (`local.LocalGroup`)) "| ActorName: " (`KismetSystemLibrary.GetDisplayName` (`local.Actor`)) "| RemainNum: " (`KismetStringLibrary.Conv_IntToString` (`KismetArrayLibrary.Array_Length` (`.Actors_3_881F6EFA4F308E3FE4AA9FB5B124018A` (break `/Game/BA_Rougelike/GameData/Structs/S_GroupActorInfo` _value_2)))))))))))))