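; Subsystem that shows on-screen direction indicators pointing toward registered actors that are off screen.
; AddDirectionTip skips hide-location actors, maps each remaining actor to a WBP_DirectionTip, and adds it to the viewport hidden if its class has a configured icon.
; On tick, each tip's position follows the actor's projected location clamped to the viewport, and its arrow rotates along the screen-space player-to-target direction.
; Tips collapse while their actor is on screen.
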(event `self.OnTick`
  (params (DeltaTime :type "Float (single-precision)"))
  ;[1 1 1] 判空
  (if (`BlueprintMapLibrary.Map_IsNotEmpty` (`self.TipWidgetMap`))
    ;[1 1 1] 遍历对照表的Key-Actor
    (bind _keys (`BlueprintMapLibrary.Map_Keys` (`self.TipWidgetMap`)))
    (for _array_element _keys
      (bind (_value _returnvalue) (`BlueprintMapLibrary.Map_Find` (`self.TipWidgetMap`) _array_element))
      ;[1 1 1] 查找对应提示UI
      (if _returnvalue
        ;[1 1 1] 设置提示在屏幕上的位置
        (`self.SetTipLocation` _array_element _value)
        ;[1 1 1] 设置提示在屏幕上的旋转
        (`self.SetTipAngle` _array_element _value)
        ;[1 1 1] 根据目标是否已经在屏幕上切换提示显示
        (if (`self.IsActorOnScreen` _array_element)
          (`self.HideTip` _value)
          (else
            (`self.ShowTip` _value)))))))

(fn `AddDirectionTip`
  (params (Actor :type "Actor Object Reference"))
  (locals (LocalActor :type "Actor Object Reference") (LocalTipWidget :type "/Game/BA_Rougelike/Blueprints/UMG/WBP_DirectionTip Object Reference"))
  (bind (_value _returnvalue) (`BlueprintMapLibrary.Map_Find` (`self.TipIconConfig`) (`GameplayStatics.GetObjectClass` (`local.LocalActor`))))
  (bind _output_get (set `local.LocalActor` Actor))
  ;[1 1 1] 有效性判断
  (`/Engine/EditorBlueprintResources/StandardMacros.IsValid` _output_get
    (:`Is Valid`
      (bind _ishidelocation (`/Game/BA_Rougelike/Blueprints/BFL/BFL_Common.IsActorHideLocation` (`local.LocalActor`)))
      (if (not _ishidelocation)
        ;[1 1 1] 创建提示UI
        (bind _returnvalue_2 (`|CreateWidget` "/Game/BA_Rougelike/Blueprints/UMG/WBP_DirectionTip.WBP_DirectionTip_C"))
        (set `local.LocalTipWidget` _returnvalue_2)
        ;[1 1 1] 添加到对照表
        (`BlueprintMapLibrary.Map_Add` (`self.TipWidgetMap`) (`local.LocalActor`) (`local.LocalTipWidget`))
        ;[1 1 1] 设置提示纹理
        (if _returnvalue
          (`/Game/BA_Rougelike/Blueprints/UMG/WBP_DirectionTip.SetTipIcon` (`local.LocalTipWidget`) _value)
          ;[1 1 1] 添加到视口
          (`UserWidget.AddToViewport` (`local.LocalTipWidget`) 0)
          ;[1 1 1] 先隐藏
          (`self.HideTip` (`local.LocalTipWidget`)))))))

(fn `HideTip`
  (params (TipWidget :type "Widget Object Reference"))
  (if (`|EnumEquality` (`Widget.GetVisibility` TipWidget) "SelfHitTestInvisible")
    (`Widget.SetVisibility` TipWidget "Collapsed")))

(fn `IsActorOnScreen`
  (params (Actor :type "Actor Object Reference"))
  (returns (ReturnValue :type Boolean))
  (bind (_returnvalue_x _returnvalue_y) (`KismetMathLibrary.BreakVector2D` (`WidgetLayoutLibrary.GetViewportSize`)))
  (bind _screenposition (`GameplayStatics.ProjectWorldToScreen` (`GameplayStatics.GetPlayerController` 0) (`Actor.K2_GetActorLocation` Actor)))
  (return (and (`KismetMathLibrary.InRange_FloatFloat` (`KismetMathLibrary.BreakVector2D` _screenposition) 0.0 _returnvalue_x) (`KismetMathLibrary.InRange_FloatFloat` (`.Y` (`KismetMathLibrary.BreakVector2D` _screenposition)) 0.0 _returnvalue_y))))

(fn `SetTipAngle`
  (params (Actor :type "Actor Object Reference") (TipWidget :type "/Game/BA_Rougelike/Blueprints/UMG/WBP_DirectionTip Object Reference"))
  (bind _outdir (`KismetMathLibrary.ToDirectionAndLength2D` (- (`GameplayStatics.ProjectWorldToScreen` (`GameplayStatics.GetPlayerController` 0) (`Actor.K2_GetActorLocation` (`GameplayStatics.GetPlayerPawn` 0))) (`GameplayStatics.ProjectWorldToScreen` (`GameplayStatics.GetPlayerController` 0) (`Actor.K2_GetActorLocation` Actor)))))
  (`Widget.SetRenderTransformAngle` (`/Game/BA_Rougelike/Blueprints/UMG/WBP_DirectionTip.DirectionImage` TipWidget) (+ (`KismetMathLibrary.DegAtan2` (`.Y` (`KismetMathLibrary.BreakVector2D` _outdir)) (`KismetMathLibrary.BreakVector2D` _outdir)) 180.0)))

(fn `SetTipLocation`
  (params (Actor :type "Actor Object Reference") (TipWidget :type "UserWidget Object Reference"))
  (bind _screenposition (`GameplayStatics.ProjectWorldToScreen` (`GameplayStatics.GetPlayerController` 0) (`Actor.K2_GetActorLocation` Actor)))
  (bind (_returnvalue_x _returnvalue_y) (`KismetMathLibrary.BreakVector2D` (- (`WidgetLayoutLibrary.GetViewportSize`) (/ (`Widget.GetDesiredSize` TipWidget) 2.0))))
  (`UserWidget.SetPositionInViewport` TipWidget (`KismetMathLibrary.MakeVector2D` (`KismetMathLibrary.FClamp` (`KismetMathLibrary.BreakVector2D` _screenposition) 0.0 _returnvalue_x) (`KismetMathLibrary.FClamp` (`.Y` (`KismetMathLibrary.BreakVector2D` _screenposition)) 0.0 _returnvalue_y)) true))

(fn `ShowTip`
  (params (TipWidget :type "Widget Object Reference"))
  (if (`|EnumEquality` (`Widget.GetVisibility` TipWidget) "Collapsed")
    (`Widget.SetVisibility` TipWidget "SelfHitTestInvisible")))