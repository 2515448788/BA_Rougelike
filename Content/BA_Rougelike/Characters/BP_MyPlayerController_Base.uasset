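; Base player controller for a roguelike that handles target lock-on for the controlled character.
; An interface sets, clears and returns the target actor, and each tick checks whether one is valid.
; With a target, control yaw smoothly interpolates toward it and the pawn follows controller yaw; without one, the character orients to its movement direction.
; The mouse cursor is hidden at BeginPlay.
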(event `self.ReceiveBeginPlay`
  (set `self.bShowMouseCursor` false))

(event `self.ReceiveTick`
  (params (DeltaSeconds :type "Float (single-precision)"))
  (set `self.Delta Seconds` DeltaSeconds)
  (bind _targetactor (`self.TargetActor`)
    (:`then`
      (`self.LookAtTargetActor` _targetactor)
      (`self.SetCharacterRotateMode` "NewEnumerator1"))
    (:`else`
      (`self.SetCharacterRotateMode` "NewEnumerator0"))))

(event `/Game/BA_Rougelike/GameData/BPI/BPI_PlayerController.Set_CurrentTarget`
  (params (TargetActor :type "Actor Object Reference"))
  (set `self.TargetActor` TargetActor))

(event `/Game/BA_Rougelike/GameData/BPI/BPI_PlayerController.Clear_CurrentTarget`
  (set `self.TargetActor` null))

(fn `Get_CurrentTarget`
  (returns (CurTarget :type "Actor Object Reference"))
  (return (`self.TargetActor`)))

(fn `LookAtTargetActor`
  (params (TargetActor :type "Actor Object Reference"))
  (bind (_returnvalue_roll _returnvalue_pitch) (`KismetMathLibrary.BreakRotator` (`self.GetControlRotation`)))
  (bind (_returnvalue_roll_2 _returnvalue_pitch_2 _returnvalue_yaw) (`KismetMathLibrary.BreakRotator` (`KismetMathLibrary.RInterpTo` (`self.K2_GetActorRotation` (`self.K2_GetPawn`)) (`KismetMathLibrary.FindLookAtRotation` (`self.K2_GetActorLocation` (`self.K2_GetPawn`)) (`self.K2_GetActorLocation` TargetActor)) (`self.Delta Seconds`) 8.0)))
  (`self.SetControlRotation` (`KismetMathLibrary.MakeRotator` _returnvalue_roll _returnvalue_pitch _returnvalue_yaw)))

(fn `SetCharacterRotateMode`
  (params (RotateMode :type "/Game/BA_Rougelike/GameData/Enums/Character/Movement/E_CharacterRotateMode Enum" :default "E_CharacterRotateMode_MAX"))
  (locals (LocalPawn :type "Pawn Object Reference") (LocalRotateMode :type "/Game/BA_Rougelike/GameData/Enums/Character/Movement/E_CharacterRotateMode Enum" :default "NewEnumerator0"))
  (bind _returnvalue (`Pawn.GetMovementComponent` (`local.LocalPawn`)))
  (set `local.LocalRotateMode` RotateMode)
  (bind _output_get (set `local.LocalPawn` (`self.K2_GetPawn`)))
  (set `Pawn.bUseControllerRotationYaw` (select `/Game/BA_Rougelike/GameData/Enums/Character/Movement/E_CharacterRotateMode` (`local.LocalRotateMode`) :`NewEnumerator1` true) _output_get)
  (`/Engine/EditorBlueprintResources/StandardMacros.IsValid` _returnvalue
    (:`Is Valid`
      (bind `_as角色移动组件` (cast `CharacterMovementComponent` _returnvalue))
      (set `CharacterMovementComponent.bOrientRotationToMovement` (select `/Game/BA_Rougelike/GameData/Enums/Character/Movement/E_CharacterRotateMode` (`local.LocalRotateMode`) :`NewEnumerator0` true) `_as角色移动组件`))))

(fn `UserConstructionScript`)