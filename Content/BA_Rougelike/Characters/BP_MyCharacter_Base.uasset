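; Base player character for a roguelike with camera-relative movement and automatic attacks on nearby enemies.
; BeginPlay sets up input, HUD and health bar, grants GAS abilities with optional input bindings, applies effects, and binds health and speed changes.
; An overlap sphere tracks "Enemy"-tagged actors; timers report the nearest to the PlayerController and start montage and looping fire sound once forward vectors roughly oppose.
; Debug inputs toggle an attribute panel and targeting visualization.
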(event `self.ReceiveBeginPlay`
  (`self.InitMappingContext`) ; 初始化输入
  (`self.InitHUD`) ; 初始化HUD
  (`self.InitHealthBar`) ; 初始化血条
  (`self.BindAttributeChangeFun`) ; 绑定属性变化回调
  (`self.InitBasicGAGE`) ; 给予基础GA 应用基础GE
  (`self.InitMoveSpeed`) ; 初始化移速
  (`self.OnBeginPlayComplete`))

(event `EnhancedInput|/Game/ThirdPerson/Input/Actions/IA_Move`
  (params (ActionValue :type "Vector2D Structure") (ElapsedSeconds :type "Float (double-precision)") (TriggeredSeconds :type "Float (double-precision)") (InputAction :type "InputAction Object Reference" :default "/Game/ThirdPerson/Input/Actions/IA_Move.IA_Move"))
  ;[1 1 1] 移动
  (:`Triggered`
    (`self.AddMovementInput` (`SceneComponent.GetRightVector` (`self.Camera`)) ActionValue_X)
    (`self.AddMovementInput` (`SceneComponent.GetForwardVector` (`self.Camera`)) ActionValue_Y)))

(event `self.TargetOverlap.OnComponentBeginOverlap`
  (params (OverlappedComponent :type "PrimitiveComponent Object Reference") (OtherActor :type "Actor Object Reference") (OtherComp :type "PrimitiveComponent Object Reference") (OtherBodyIndex :type Integer) (bFromSweep :type Boolean) (SweepResult :type "HitResult Structure (by ref)"))
  ;[1 1 1] 重叠开始
  (`self.IsTargetExist` OtherActor ; 确保不是已存在
    (:`false`
      (`self.IsEnemy` OtherActor ; 是否有敌人标签
        (:`真`
          (`KismetArrayLibrary.Array_AddUnique` (`self.TargetList`) OtherActor) ; 加入到列表
          (`self.IsTargetListEmpty` ; 目标列表是否为空
            (:`false`
              (`self.StartLoopSetCurTarget`) ; 开启朝向目标循环
              (`self.StartLoopAttacking`) ; 开始循环攻击
            )))))))

(event `self.TargetOverlap.OnComponentEndOverlap`
  (params (OverlappedComponent :type "PrimitiveComponent Object Reference") (OtherActor :type "Actor Object Reference") (OtherComp :type "PrimitiveComponent Object Reference") (OtherBodyIndex :type Integer))
  ;[1 1 1] 重叠结束
  (`self.IsTargetExist` OtherActor ; 确保已存在
    (:`真`
      (`KismetArrayLibrary.Array_RemoveItem` (`self.TargetList`) OtherActor) ; 从列表中移除
      (`self.IsTargetListEmpty` ; 目标列表是否为空
        (:`真`
          (`self.EndLoodSetCurTarget`) ; 结束朝向目标循环
          (`self.ClearCurTarget`) ; 清除玩家控制器当前目标
          (`self.EndLoopAttacking`) ; 结束循环攻击
        )))))

(event `self.ReceiveTick`
  (params (DeltaSeconds :type "Float (single-precision)"))
  (`self.Debug_TargetSystem`))

(event `EnhancedInput|/Game/BA_Rougelike/Input/Actions/IA_Debug_ShowAttributeSet`
  (params (ActionValue :type Boolean) (ElapsedSeconds :type "Float (double-precision)") (TriggeredSeconds :type "Float (double-precision)") (InputAction :type "InputAction Object Reference" :default "/Game/BA_Rougelike/Input/Actions/IA_Debug_ShowAttributeSet.IA_Debug_ShowAttributeSet"))
  ;[1 1 1] 调试-显示所有属性
  (:`Started`
    (switch `/Game/BA_Rougelike/GameData/Enums/Character/Debug/E_DebugMode` (`self.DebugMode_AttributeSet`)
      (:`NewEnumerator2`
        (set `self.DebugMode_AttributeSet` "NewEnumerator1")
        (bind _returnvalue (`/Game/BA_Rougelike/Blueprints/UMG/WBP_UserBaseCanvas.PushWidget` (`self.UserBaseCanvas`) "/Game/BA_Rougelike/Blueprints/UMG/Debug/CAW_AttributeSetPanel.CAW_AttributeSetPanel_C"))
        (set `self.AttributeSetPanel` _returnvalue)
        (`self.SetShowMouseCursor` true))
      (:`NewEnumerator1`
        (set `self.DebugMode_AttributeSet` "NewEnumerator2")
        (bind _attributesetpanel (`self.AttributeSetPanel`)
          (:`then`
            (`/Game/BA_Rougelike/Blueprints/UMG/WBP_UserBaseCanvas.RemoveWidget` (`self.UserBaseCanvas`) _attributesetpanel)
            (`self.SetShowMouseCursor` false))
          (:`else`))))))

(event `EnhancedInput|/Game/BA_Rougelike/Input/Actions/IA_Debug_ShowTargetSystemRadius`
  (params (ActionValue :type Boolean) (ElapsedSeconds :type "Float (double-precision)") (TriggeredSeconds :type "Float (double-precision)") (InputAction :type "InputAction Object Reference" :default "/Game/BA_Rougelike/Input/Actions/IA_Debug_ShowTargetSystemRadius.IA_Debug_ShowTargetSystemRadius"))
  (:`Triggered`
    (switch `/Game/BA_Rougelike/GameData/Enums/Character/Debug/E_DebugMode` (`self.DebugMode_TargetSystem`)
      (:`NewEnumerator2`
        (set `self.DebugMode_TargetSystem` "NewEnumerator1"))
      (:`NewEnumerator1`
        (set `self.DebugMode_TargetSystem` "NewEnumerator2")))))

(fn `BindAttributeChangeFun`
  (add `self.HealthChangedEvent` (`|CreateDelegate` :!event `OnHealthChanged`))
  (add `self.MoveSpeedChangedEvent` (`|CreateDelegate` :!event `OnMoveSpeedChanged`)))

(fn `ClearCurTarget`
  (message `/Game/BA_Rougelike/GameData/BPI/BPI_PlayerController.Clear_CurrentTarget` (`self.GetLocalViewingPlayerController`))
  (set `self.CurrentTarget` null))

(fn `Debug_TargetSystem`
  (if (`|EnumEquality` (`self.DebugMode_TargetSystem`) "NewEnumerator1")
    (`KismetSystemLibrary.DrawDebugCircle` (`self.K2_GetActorLocation`) (`SphereComponent.SphereRadius` (`self.TargetOverlap`)) 36 (struct :`G` 0.286018 :`B` 1.0 :`A` 1.0) 0.0 2.0 (0.0 1.0 0.0) (1.0 0.0 0.0))
    (bind _currenttarget (`self.CurrentTarget`)
      (:`then`
        (`KismetSystemLibrary.DrawDebugArrow` (`self.K2_GetActorLocation`) (`self.K2_GetActorLocation` _currenttarget) 10.0 (struct :`G` 1.0 :`B` 0.077964 :`A` 1.0) 0.0 2.0))
      (:`else`))))

(fn `EndLoodSetCurTarget`
  (if (`KismetSystemLibrary.K2_IsValidTimerHandle` (`self.LoopSetCurTargetTimer`))
    (`KismetSystemLibrary.K2_ClearAndInvalidateTimerHandle` (`self.LoopSetCurTargetTimer`))))

(fn `EndLoopAttacking`
  (`|ExecutionSequence`
    (:`then_0`
      ;[1 1 1] 停止蒙太奇
      (`self.StopAnimMontage` (`self.AttackMontage`))
      (set `self.IsAlreadyAttacking` false)
      ;;[1 1 1] 结束等待攻击定时器
      (`KismetSystemLibrary.K2_ClearAndInvalidateTimerHandle` (`self.WaitForAttackHandel`)))
    (:`then_1`
      ;[1 1 1] 停止播放开火音效
      (`AudioComponent.FadeOut` (`self.LoopFireSoundComp`) 0.15 0.0 "Linear"))))

(fn `Get_AttackMontage`
  (returns (Montage :type "AnimMontage Object Reference"))
  (return (`self.AttackMontage`)))

(fn `Get_BaseCanvas`
  (returns (UserBaseCanvas :type "/Game/BA_Rougelike/Blueprints/UMG/WBP_UserBaseCanvas Object Reference"))
  (return (`self.UserBaseCanvas`)))

(fn `InitAimPoint`
  (`SceneComponent.K2_AttachToComponent` (`self.AimPoint`) (`self.Mesh`) (`self.AimSocketName`) "SnapToTarget" "SnapToTarget" "SnapToTarget" true))

(fn `InitBasicGAGE`
  (`|ExecutionSequence`
    (:`then_0`
      (bind _keys (`BlueprintMapLibrary.Map_Keys` (`self.BasicGAList`)))
      (for _array_element _keys
        (bind (_ability _level) (break `/Game/BA_Rougelike/GameData/Structs/S_BasicGA` _array_element))
        (bind _returnvalue (`AbilitySystemComponent.K2_GiveAbility` (`self.EnhancedInputAbilitySystem`) _ability _level -1))
        (bind (_value _returnvalue_2) (`BlueprintMapLibrary.Map_Find` (`self.BasicGAList`) _array_element))
        (if _returnvalue_2
          (`/Engine/EditorBlueprintResources/StandardMacros.IsValid` _value
            (:`Is Valid`
              (`EnhancedInputAbilitySystem.SetInputBinding` (`self.EnhancedInputAbilitySystem`) _value _returnvalue))))))
    (:`then_1`
      (bind _keys_2 (`BlueprintMapLibrary.Map_Keys` (`self.BasicGEtList`)))
      (for _array_element_2 _keys_2
        (bind (_value_2 _returnvalue_3) (`BlueprintMapLibrary.Map_Find` (`self.BasicGEtList`) _array_element_2))
        (if _returnvalue_3
          (`AbilitySystemComponent.BP_ApplyGameplayEffectToSelf` :`self` (`self.EnhancedInputAbilitySystem`) :`GameplayEffectClass` _array_element_2 :`Level` _value_2))))))

(fn `InitHealthBar`
  (bind (_bsuccessfullyfoundattribute _returnvalue) (`AbilitySystemBlueprintLibrary.GetFloatAttribute` self (struct :`AttributeName` "MaxHealth" :`Attribute` "/Script/BA_Rougelike.MyAttributeSet_Character:MaxHealth" :`AttributeOwner` "/Script/CoreUObject.Class'/Script/BA_Rougelike.MyAttributeSet_Character'")))
  (bind (_bsuccessfullyfoundattribute_2 _returnvalue_2) (`AbilitySystemBlueprintLibrary.GetFloatAttribute` self (struct :`AttributeName` "Health" :`Attribute` "/Script/BA_Rougelike.MyAttributeSet_Character:Health" :`AttributeOwner` "/Script/CoreUObject.Class'/Script/BA_Rougelike.MyAttributeSet_Character'")))
  (if (and _bsuccessfullyfoundattribute_2 _bsuccessfullyfoundattribute)
    (`/Game/BA_Rougelike/Blueprints/Components/HealthBar/BPC_HealthBar.InitHealthBar` (`self.BPC_HealthBar`) _returnvalue_2 _returnvalue)
    (`KismetSystemLibrary.PrintString` "初始化血条")))

(fn `InitHUD`
  (bind _returnvalue (`|CreateWidget` "/Game/BA_Rougelike/Blueprints/UMG/WBP_UserBaseCanvas.WBP_UserBaseCanvas_C" (`GameplayStatics.GetPlayerController` 0)))
  (bind _output_get (set `self.UserBaseCanvas` _returnvalue))
  (`UserWidget.AddToViewport` _output_get 0))

(fn `InitMappingContext`
  (bind `_as玩家控制器` (cast `PlayerController` (`self.GetController`)))
  (bind _returnvalue (pcsubsystem `EnhancedInputLocalPlayerSubsystem` `_as玩家控制器`))
  (`/Engine/EditorBlueprintResources/StandardMacros.IsValid` _returnvalue
    (:`Is Valid`
      (`EnhancedInputSubsystemInterface.AddMappingContext` _returnvalue "/Game/BA_Rougelike/Input/IMC_MyDefault.IMC_MyDefault" 0 (struct)))))

(fn `InitMoveSpeed`
  (bind (_bsuccessfullyfoundattribute _returnvalue) (`AbilitySystemBlueprintLibrary.GetFloatAttribute` self (struct :`AttributeName` "MoveSpeed" :`Attribute` "/Script/BA_Rougelike.MyAttributeSet_Character:MoveSpeed" :`AttributeOwner` "/Script/CoreUObject.Class'/Script/BA_Rougelike.MyAttributeSet_Character'")))
  (if _bsuccessfullyfoundattribute
    (`self.OnMoveSpeedChanged` _returnvalue)
    (`KismetSystemLibrary.PrintString` (`KismetStringLibrary.Concat_StrStr` "初始化移速" (`KismetStringLibrary.Conv_DoubleToString` _returnvalue)))
    (else
      (`KismetSystemLibrary.PrintString` "移速初始化失败"))))

(fn `OnHealthChanged`
  (params (NewValue :type "Float (double-precision)"))
  (`/Game/BA_Rougelike/Blueprints/Components/HealthBar/BPC_HealthBar.UpdateCurHealth` (`self.BPC_HealthBar`) NewValue))

(fn `OnMoveSpeedChanged`
  (params (NewValue :type "Float (double-precision)"))
  (set `CharacterMovementComponent.MaxWalkSpeed` NewValue (`self.CharacterMovement`)))

(fn `SetCurTarget`
  (locals (LocalMinDistance :type "Float (single-precision)" :default 0.0) (LocalCurTarget :type "Actor Object Reference"))
  (bind _returnvalue (`self.GetLocalViewingPlayerController`))
  (`self.IsTargetListEmpty`
    (:`false`
      (set `local.LocalMinDistance` 99999999999.0)
      (for _array_element (`self.TargetList`)
        (bind _returnvalue_2 (`self.GetDistanceTo` _array_element))
        (if (<= _returnvalue_2 (`local.LocalMinDistance`))
          (set `local.LocalMinDistance` _returnvalue_2)
          (set `local.LocalCurTarget` _array_element)))
      (bind _localcurtarget (`local.LocalCurTarget`)
        (:`then`
          (bind _curtarget (message `/Game/BA_Rougelike/GameData/BPI/BPI_PlayerController.Get_CurrentTarget` _returnvalue))
          (if (!= _curtarget _localcurtarget)
            (bind _output_get (set `self.CurrentTarget` (`local.LocalCurTarget`)))
            (message `/Game/BA_Rougelike/GameData/BPI/BPI_PlayerController.Set_CurrentTarget` _returnvalue _output_get)))
        (:`else`)))))

(fn `SetShowMouseCursor`
  (params (`显示鼠标光标` :type Boolean))
  (set `PlayerController.bShowMouseCursor` `显示鼠标光标` (`GameplayStatics.GetPlayerController` 0)))

(fn `StartLoopAttacking`
  (if (not (`self.IsAlreadyAttacking`))
    ;[1 1 1] 循环等待播放攻击蒙太奇
    (if (not (`KismetSystemLibrary.K2_IsTimerActiveHandle` (`self.WaitForAttackHandel`)))
      (bind _returnvalue (`KismetSystemLibrary.K2_SetTimer` null "WaitForAttack" 0.1 true))
      (set `self.WaitForAttackHandel` _returnvalue))))

(fn `StartLoopSetCurTarget`
  (if (not (`KismetSystemLibrary.K2_IsTimerActiveHandle` (`self.LoopSetCurTargetTimer`)))
    (bind _returnvalue (`KismetSystemLibrary.K2_SetTimer` null "SetCurTarget" 0.1 true))
    (set `self.LoopSetCurTargetTimer` _returnvalue)))

(fn `UserConstructionScript`
  (`self.InitAimPoint`))

(fn `WaitForAttack`
  (bind _currenttarget (`self.CurrentTarget`)
    (:`then`
      (if (`KismetMathLibrary.InRange_FloatFloat` (`KismetMathLibrary.Dot_VectorVector` (`KismetMathLibrary.GetForwardVector` (`self.K2_GetActorRotation` _currenttarget)) (`KismetMathLibrary.GetForwardVector` (`self.K2_GetActorRotation`))) -1.0 -0.8)
        (`|ExecutionSequence`
          (:`then_0`
            ;[1 1 1] 循环开火蒙太奇
            (`self.PlayAnimMontage` (`self.AttackMontage`))
            (set `self.IsAlreadyAttacking` true)
            ;;[1 1 1] 结束等待攻击定时器
            (`KismetSystemLibrary.K2_ClearAndInvalidateTimerHandle` (`self.WaitForAttackHandel`)))
          (:`then_1`
            ;[1 1 1] 循环开火音效
            (`AudioComponent.Sound` (`self.LoopFireSoundComp`)
              (:`then`
                (if (not (`AudioComponent.IsPlaying` (`self.LoopFireSoundComp`)))
                  (`AudioComponent.Play` (`self.LoopFireSoundComp`) 0.0)))
              (:`else`))))))
    (:`else`)))