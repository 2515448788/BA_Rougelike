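; Base enemy character Blueprint for a roguelike, providing health, movement speed and a normal melee-style attack through interface events.
; A normal attack is gated by a cooldown: a timeline rotates the enemy toward the player, then plays the attack montage and waits out the attack interval.
; Damage lowers clamped health and updates a health bar component.
; Getters expose attack stats, attack state and patrol points.
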(event `self.ReceiveBeginPlay`
  (`self.InitHealthBar`))

(event `/Game/BA_Rougelike/GameData/BPI/BPI_AI.NormalAttack`
  ;[1 1 1] 普通攻击
  (if (not (`self.IsAttackCooldown`))
    (set `self.IsAttackCooldown` true) ; 设置冷却
    (bind (_direction _alpha) (`Timeline|TL_RotateToPlayer` :!via `PlayFromStart`)
      (:`Update`
        (`self.RotateToPlayer` _alpha))
      (:`Finished`
        (`self.PlayAnimMontage` (`self.AttackMontage`))
        ;;[1 1 1] 攻击冷却逻辑
        (`KismetSystemLibrary.Delay` (`self.AttackInterval`))
        (set `self.IsAttackCooldown` false)))))

(event `/Game/BA_Rougelike/GameData/BPI/BPI_AI.SetAttackState`
  (params (IsAttackState :type Boolean))
  ;[1 1 1] 攻击状态控制
  (set `self.IsInAttackState` IsAttackState))

(event `self.ReceiveAnyDamage`
  (params (Damage :type "Float (single-precision)") (DamageType :type "DamageType Object Reference") (InstigatedBy :type "Controller Object Reference") (DamageCauser :type "Actor Object Reference"))
  (bind _output_get (set `self.CurHealth` (`KismetMathLibrary.FClamp` (- (`self.CurHealth`) Damage) 0.0 (`self.MaxHealth`))))
  (`/Game/BA_Rougelike/Blueprints/Components/HealthBar/BPC_HealthBar.UpdateCurHealth` (`self.BPC_HealthBar`) _output_get))

(fn `Get_AttackDamage`
  (returns (AttackDamage :type "Float (double-precision)"))
  (return (`self.AttackDamage`)))

(fn `Get_AttackInterval`
  (returns (AttackInterval :type "Float (double-precision)"))
  (return (`self.AttackInterval`)))

(fn `Get_AttackMontage`
  (returns (Montage :type "AnimMontage Object Reference"))
  (return (`self.AttackMontage`)))

(fn `Get_AttackRange`
  (returns (Range :type "Float (double-precision)"))
  (return (`self.AttackRange`)))

(fn `Get_IsInAttackState`
  (returns (IsInAttackState :type Boolean))
  (return (`self.IsInAttackState`)))

(fn `Get_MoveSpeed`
  (returns (MoveSpeed :type "Float (double-precision)"))
  (return (`self.MoveSpeed`)))

(fn `Get_PatrolList`
  (returns (List :type "Array of Actor Object Reference"))
  (return (`self.PatrolPointList`)))

(fn `InitHealthBar`
  (`/Game/BA_Rougelike/Blueprints/Components/HealthBar/BPC_HealthBar.InitHealthBar` (`self.BPC_HealthBar`) (`self.CurHealth`) (`self.MaxHealth`)))

(fn `RotateToPlayer`
  (params (Alpha :type "Float (single-precision)"))
  (`self.K2_SetActorRotation` (`KismetMathLibrary.RLerp` (`self.K2_GetActorRotation`) (`KismetMathLibrary.FindLookAtRotation` (`self.K2_GetActorLocation`) (`self.K2_GetActorLocation` (`GameplayStatics.GetPlayerPawn` 0))) Alpha true)))

(fn `UserConstructionScript`
  ;[1 1 1] 初始化移动速度
  (set `CharacterMovementComponent.MaxWalkSpeed` (`self.MoveSpeed`) (`self.CharacterMovement`)))