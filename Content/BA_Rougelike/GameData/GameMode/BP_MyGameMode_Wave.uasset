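; Wave game mode that runs timed enemy waves and updates a wave-info widget, starting once the player character finishes initializing.
; A looping one-second countdown advances waves, each read from a WaveData DataTable row named by wave index.
; Sub-waves chain sequentially: a timer runs an EQS query around the player, then its finish callback spawns pooled enemies with Niagara FX at random result locations and schedules the next sub-wave.
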(event `self.ReceiveBeginPlay`
  (`parent.ReceiveBeginPlay`)
  ;[1 1 1] 大波次索引从1开始 小波次索引从0开始（数组索引从0开始）
  (set `self.CurWaveIndex` 1)
  (set `self.CurSubWaveIndex` 0)
  ;[1 1 1] 等待玩家初始化完毕
  (bind _asbp_my_character_base (cast `/Game/BA_Rougelike/Characters/BP_MyCharacter_Base` (`GameplayStatics.GetPlayerPawn` 0)))
  (add `/Game/BA_Rougelike/Characters/BP_MyCharacter_Base.OnBeginPlayComplete` _asbp_my_character_base (`|CreateDelegate` :!event `OnPlayerBeginPlayComplete`)))

(fn `AddWaveWidget`
  (bind _returnvalue (`|CreateWidget` "/Game/BA_Rougelike/Blueprints/UMG/WBP_WaveInfo.WBP_WaveInfo_C" (`GameplayStatics.GetPlayerController` 0)))
  (bind _output_get (set `self.WaveWidget` _returnvalue))
  (`UserWidget.AddToViewport` _output_get 0)
  ;[1 1 1] 初始化倒计时-默认是第一波
  (bind _countdown (`self.GetCurWaveInfo`)
    (:`Success`
      (message `/Game/BA_Rougelike/GameData/BPI/BPI_WaveWidget.UpdateCountDown` (`self.WaveWidget`) _countdown))))

(fn `GetCurWaveAsName`
  (returns (ReturnValue :type Name))
  (return (`KismetStringLibrary.Conv_StringToName` (`KismetStringLibrary.Conv_IntToString` (`self.CurWaveIndex`)))))

(fn `LoopWaveCountdown`
  (`|ExecutionSequence`
    (:`then_0`
      (bind _result (`/Engine/EditorBlueprintResources/StandardMacros.DecrementInt` (`self.CurCountdownTime`)) ; 倒计时自减
        (:`  `
          (if (== _result 0)
            (`KismetSystemLibrary.K2_ClearAndInvalidateTimerHandle` (`self.CountdownHandel`))
            ;[1 1 1] 主波次索引自增 再次开始当前波次倒计时并生成主波次敌人
            (`/Engine/EditorBlueprintResources/StandardMacros.IncrementInt` (`self.CurWaveIndex`)
              (:`  `
                (`self.StartWaveCountdown`)))))))
    (:`then_1`
      ;[1 1 1] 更新当前波次倒计时
      (bind _wavewidget (`self.WaveWidget`)
        (:`then`
          (message `/Game/BA_Rougelike/GameData/BPI/BPI_WaveWidget.UpdateCountDown` _wavewidget (`self.CurCountdownTime`)))
        (:`else`)))))

(fn `OnEQSQueryFinished`
  (params (QueryInstance :type "EnvQueryInstanceBlueprintWrapper Object Reference") (QueryStatus :type "EEnvQueryStatus Enum" :default "Processing"))
  (locals (Loc :type "Vector Structure") (LocalResultLocations :type "Array of Vector Structure"))
  ;[1 1 1] 子波次敌人生成逻辑
  (bind (_resultlocations _returnvalue) (`EnvQueryInstanceBlueprintWrapper.GetQueryResultsAsLocations` QueryInstance))
  (bind _output_get (set `local.LocalResultLocations` _resultlocations))
  (if _returnvalue
    (for _ (range 1 (+ (`KismetMathLibrary.Min` (`KismetArrayLibrary.Array_Length` _output_get) (`.SpawnNum_9_A119D03942ED010821A457BA7566773A` (break `/Game/BA_Rougelike/GameData/Structs/S_SubWaveInfo` (`self.SubWaveInfo`)))) 1))
      (bind _output_get_2 (set `local.Loc` (`KismetArrayLibrary.Array_Random` (`local.LocalResultLocations`))))
      (`self.SapwnFX` _output_get_2)
      (`PoolSubsystem.SpawnFromPool` :`self` (subsystem `PoolSubsystem`) :`PoolClass` (`.SpawnActorClass_6_B4A9A15F45E58F6D6C863EA6C6EEE4C5` (break `/Game/BA_Rougelike/GameData/Structs/S_SubWaveInfo` (`self.SubWaveInfo`))) :`Location` (`local.Loc`)))
    ;[1 1 1] 事件解绑
    (remove `EnvQueryInstanceBlueprintWrapper.OnQueryFinishedEvent` QueryInstance (`|CreateDelegate` :!event `OnEQSQueryFinished`))
    ;[1 1 1] 子波次自增 开始生成下一子波次敌人
    (`/Engine/EditorBlueprintResources/StandardMacros.IncrementInt` (`self.CurSubWaveIndex`)
      (:`  `
        (`self.StartSubWaveSpawn` (`self.CurWaveInfo`))))))

(fn `OnPlayerBeginPlayComplete`
  (`self.AddWaveWidget`)
  (`self.StartWaveCountdown`))

(fn `SapwnFX`
  (params (Loc :type "Vector Structure"))
  (`NiagaraFunctionLibrary.SpawnSystemAtLocation` "/Game/BA_Rougelike/Niagara/NS_EnemySpawn.NS_EnemySpawn" Loc (struct) (1.0 1.0 1.0) true true "AutoRelease"))

(fn `StartCurWaveSpawn`
  ;[1 1 1] 设置当前波次所有的定时器
  (bind (_countdown _curwaveinfo) (`self.GetCurWaveInfo`)
    (:`Success`
      (set `self.CurSubWaveIndex` 0) ; 每次开始新的主波次都重置子波次索引为0
      (bind _output_get (set `self.CurWaveInfo` _curwaveinfo))
      (`self.StartSubWaveSpawn` _output_get))))

(fn `StartEQSQuery`
  (bind _returnvalue (`EnvQueryManager.RunEQSQuery` "/Game/BA_Rougelike/AI/EQS/EQS_Player.EQS_Player" (`GameplayStatics.GetPlayerPawn` 0) "AllMatching"))
  (add `EnvQueryInstanceBlueprintWrapper.OnQueryFinishedEvent` _returnvalue (`|CreateDelegate` :!event `OnEQSQueryFinished`)))

(fn `StartSubWaveSpawn`
  (params (CurWaveInfo :type "Array of /Game/BA_Rougelike/GameData/Structs/S_SubWaveInfo Structure (by ref)"))
  (bind _subwaveinfo (`self.GetSubWaveInfo` CurWaveInfo)
    (:`Success`
      (`|ExecutionSequence`
        (:`then_0`
          (bind _output_get (set `self.SubWaveInfo` _subwaveinfo))
          (`KismetSystemLibrary.K2_SetTimer` null "StartEQSQuery" (`.SpawnTimeForCurWave_3_0A3AE45441C26C61157B06B02B543FF3` (break `/Game/BA_Rougelike/GameData/Structs/S_SubWaveInfo` _output_get))) ; 开始EQS查询和生成敌人
        )
        (:`then_1`
          ;[1 1 1] 更新子波次UI
          (message `/Game/BA_Rougelike/GameData/BPI/BPI_WaveWidget.UpdateSubWaveIndex` (`self.WaveWidget`) (`self.CurSubWaveIndex`)))))))

(fn `StartWaveCountdown`
  (`|ExecutionSequence`
    (:`then_0`
      ;[1 1 1] 更新UI和主波次索引
      (bind _wavewidget (`self.WaveWidget`)
        (:`then`
          (message `/Game/BA_Rougelike/GameData/BPI/BPI_WaveWidget.UpdateWaveIndex` _wavewidget (`self.CurWaveIndex`)) ; 更新一次波次索引
          (bind _countdown (`self.GetCurWaveInfo`)
            (:`Success`
              (set `self.CurCountdownTime` _countdown)
              ;;[1 1 1] 当前波次倒计时
              (`KismetSystemLibrary.K2_ClearAndInvalidateTimerHandle` (`self.CountdownHandel`))
              (bind _returnvalue (`KismetSystemLibrary.K2_SetTimer` null "LoopWaveCountdown" 1.0 true))
              (set `self.CountdownHandel` _returnvalue))))
        (:`else`)))
    (:`then_1`
      (`self.StartCurWaveSpawn`) ; 开始生成当前主波次敌人
    )))

(fn `UserConstructionScript`
  (`parent.UserConstructionScript`))